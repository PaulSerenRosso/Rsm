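; BP_JeremieReborn is an AI creature that gives audio feedback as it detects and loses prisoner players.
; It starts breathing audio on BeginPlay, and alert changes notify the affected BP_PrisonnerDD through ClientOnAlert.
; Multicast events drive the chase and end-of-alert audio, while losing sight triggers a roar after a delay.
; Manager door interactions only print debug text.
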(event `self.ReceiveBeginPlay`
  (`AudioComponent.Play` (`self.AudioBreath`) 0.0))

(event `self.BP_OnAlert`
  (params (Target :type "Prisoner Object Reference"))
  (bind _asbp_prisonner_dd (cast `/Game/Blueprints/Characters/BP_PrisonnerDD` Target))
  (`/Game/Blueprints/Characters/BP_PrisonnerDD.Client_OnAlert` _asbp_prisonner_dd true)
  (`self.Multicast_OnAlert`))

(event `Multicast_OnAlert`
  (bind _alertaudio (`self.AlertAudio`))
  (if (not (`AudioComponent.IsPlaying` _alertaudio))
    (`AudioComponent.SetSound` _alertaudio (`self.AudioChase`))
    (`AudioComponent.Play` _alertaudio 0.0)))

(event `self.OnLostSighPlayer`
  (params (Target :type "Prisoner Object Reference"))
  (bind _alertaudio (`self.AlertAudio`))
  (bind _asbp_prisonner_dd (cast `/Game/Blueprints/Characters/BP_PrisonnerDD` Target))
  (`/Game/Blueprints/Characters/BP_PrisonnerDD.Client_OnAlert` _asbp_prisonner_dd false)
  (`KismetSystemLibrary.Delay` 10.0)
  (`AudioComponent.SetSound` _alertaudio "/Game/Sounds/SoundWave/Jeremie/Roar.Roar")
  (`AudioComponent.Play` _alertaudio 0.0))

(event `self.OnEndAlert`
  (params (Target :type "Prisoner Object Reference"))
  (`self.Multicast_OnEndAlert`))

(event `Multicast_OnEndAlert`
  (bind _alertaudio (`self.AlertAudio`))
  (if (`AudioComponent.IsPlaying` _alertaudio)
    (`AudioComponent.Stop` _alertaudio)
    (else
      (`AudioComponent.SetSound` _alertaudio "/Game/Sounds/SoundWave/Jeremie/Roar.Roar")))
  (`AudioComponent.Play` _alertaudio 0.0))

(event `self.BP_OnInteractWithManagerDoor`
  (params (ManagerDoor :type "ManagerDoor Object Reference") (IsExit :type Boolean))
  (`KismetSystemLibrary.PrintString` (`KismetStringLibrary.Concat_StrStr` (`KismetSystemLibrary.GetDisplayName` ManagerDoor) "      " (`KismetStringLibrary.Conv_BoolToString` IsExit))))

(fn `UserConstructionScript`)