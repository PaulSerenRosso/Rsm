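; Hearing neighbour AI character that drives a proximity screen or material effect through the player's Material Parameter Collection.
; Sphere overlap events toggle IsClose after a class check.
; While close, Tick converts distance to the first overlapping actor, relative to sphere radius, into a clamped EntitiesCloseIntensity in MPC_Player and debug-prints it.
; Footstep audio logic based on ground movement exists but is disconnected.
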(event `self.Sphere.OnComponentBeginOverlap`
  (params (OverlappedComponent :type "PrimitiveComponent Object Reference") (OtherActor :type "Actor Object Reference") (OtherComp :type "PrimitiveComponent Object Reference") (OtherBodyIndex :type Integer) (bFromSweep :type Boolean) (SweepResult :type "HitResult Structure (by ref)"))
  (if (== (`GameplayStatics.GetObjectClass` OverlappedComponent) null)
    (set `self.IsClose` true)))

(event `self.ReceiveTick`
  (params (DeltaSeconds :type "Float (single-precision)"))
  (if (`self.IsClose`)
    (bind _output_get (set `self.EffectPlayerIntensity` (`KismetMathLibrary.FClamp` (- 1.0 (/ (`self.GetDistanceTo` (`|GetArrayItem` (`PrimitiveComponent.GetOverlappingActors` (`self.Overlapped Component`) null)) self) (`SphereComponent.SphereRadius` (`self.Sphere`)))))))
    (`KismetMaterialLibrary.SetScalarParameterValue` "/Game/Art/Characters/CharacterPlayer/Materials/MPC_Player.MPC_Player" "EntitiesCloseIntensity" _output_get)
    (`KismetSystemLibrary.PrintString` (`KismetStringLibrary.Conv_DoubleToString` (`self.EffectPlayerIntensity`)))))

(event `self.Sphere.OnComponentEndOverlap`
  (params (OverlappedComponent :type "PrimitiveComponent Object Reference") (OtherActor :type "Actor Object Reference") (OtherComp :type "PrimitiveComponent Object Reference") (OtherBodyIndex :type Integer))
  (if (== (`GameplayStatics.GetObjectClass` OverlappedComponent) null)
    (set `self.IsClose` false)))

(fn `UserConstructionScript`)