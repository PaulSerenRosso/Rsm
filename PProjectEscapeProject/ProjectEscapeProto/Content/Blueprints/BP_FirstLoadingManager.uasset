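; BP_FirstLoadingManager runs the first-launch flow, from name creation through initial loading to the Menu level.
; On BeginPlay it shows the WBP_CreateName widget with the mouse cursor and, shortly after selection completes, calls BeginInitCPP.
; The BeginInit event swaps that widget for WBP_FirstLoadingWidget, and EndInit opens Menu.
; The initialization work itself lies outside this graph, behind BeginInitCPP.
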(event `self.ReceiveBeginPlay`
  (bind _returnvalue (`|CreateWidget` "/Game/Blueprints/Widgets/WBP_CreateName.WBP_CreateName_C"))
  (add `/Game/Blueprints/Widgets/WBP_CreateName.SelectionCompleted` _returnvalue (delegate `SelectionCompleted_Event`))
  (`UserWidget.AddToViewport` _returnvalue 0)
  (set `PlayerController.bShowMouseCursor` true (`GameplayStatics.GetPlayerController` 0)))

(event `SelectionCompleted_Event`
  (`KismetSystemLibrary.Delay` 0.2)
  (`self.BeginInitCPP`))

(event `self.BP_BeginInit`
  (bind _returnvalue (`|CreateWidget` "/Game/Blueprints/Widgets/SubWidgets/WBP_FirstLoadingWidget.WBP_FirstLoadingWidget_C"))
  (`UserWidget.AddToViewport` _returnvalue 0)
  (`Widget.RemoveFromParent` (stale `self.ReceiveBeginPlay` _returnvalue)))

(event `self.BP_EndInit`
  (`GameplayStatics.OpenLevelBySoftObjectPtr` "/Game/Levels/Menu.Menu"))

(fn `UserConstructionScript`)