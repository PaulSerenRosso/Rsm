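; Network manager that hosts and joins online multiplayer sessions through short room codes, using Advanced Sessions-style nodes.
; HostSession copies a random six-character key to the clipboard, publishes it as the GAMEKEY session setting, then opens the level as a listen server.
; FindByKeycode searches internet sessions for a matching GAMEKEY and joins it, reporting wrong-code, search or join failures through FailedToPerform.
; Both paths store the room code in OnlineGameInstance.
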(event `HostSession`
  (bind _returnvalue (`FunctionsUtilities.CopyValueToClip` (`FunctionsUtilities.GetRandomKey` 6)))
  (`CreateSessionCallbackProxyAdvanced.CreateAdvancedSession` (`|MakeArray` (`AdvancedSessionsLibrary.MakeLiteralSessionPropertyString` "GAMEKEY" _returnvalue)) (`GameplayStatics.GetPlayerController` 0) (`OnlineGameInstance.NbPlayersNeedToPlay` (cast `OnlineGameInstance` (`GameplayStatics.GetGameInstance`) :!pure true))
    (:`OnSuccess`
      (set `OnlineGameInstance.RoomCode` _returnvalue (cast `OnlineGameInstance` (`GameplayStatics.GetGameInstance`) :!pure true))
      (`KismetSystemLibrary.Delay` 0.2)
      (`GameplayStatics.OpenLevelBySoftObjectPtr` (`self.Level`) true "listen")
      (`WidgetBlueprintLibrary.SetInputMode_GameOnly` (`GameplayStatics.GetPlayerController` 0)))
    (:`OnFailure`
      (`KismetSystemLibrary.PrintString` "Fail to create Session" true true (struct :`R` 1.0 :`G` 0.012606 :`A` 1.0) 20.0))))

(event `FindByKeycode`
  (params (Keycode :type String))
  (bind _returnvalue (`GameplayStatics.GetPlayerController` 0))
  (set `self.CanBePrintError` true)
  (bind _results (`FindSessionsCallbackProxy.FindSessions` (`GameplayStatics.GetPlayerController` 0) 100)
    (:`OnSuccess`
      (for _array_element _results
        (bind _extrasettings (`AdvancedSessionsLibrary.GetExtraSettings` _array_element))
        (bind _settingvalue (`AdvancedSessionsLibrary.GetSessionPropertyString` _extrasettings "GAMEKEY") ; Check if this session has the property
          (:`Found`
            (if (`KismetStringLibrary.EqualEqual_StrStr` _settingvalue Keycode)
              (set `self.CanBePrintError` false)
              (set `OnlineGameInstance.RoomCode` Keycode (cast `OnlineGameInstance` (`GameplayStatics.GetGameInstance`) :!pure true))
              (`JoinSessionCallbackProxy.JoinSession` _returnvalue _returnvalue _array_element
                (:`OnFailure`
                  (`self.FailedToPerform` "cant't be able to join")))))))
      (if (`self.CanBePrintError`)
        (`self.FailedToPerform` "Wrong Code")))
    (:`OnFailure`
      (`self.FailedToPerform` "Internet connection Issues"))))

(fn `UserConstructionScript`)