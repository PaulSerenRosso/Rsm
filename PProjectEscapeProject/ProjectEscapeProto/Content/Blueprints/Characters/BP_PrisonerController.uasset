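; Player controller for the prisoner character in a networked game, handling local UI, input modes and player feedback.
; Death and respawn events show and remove a restart widget, while end-game events display the winner and GameState leaderboard, with a back-to-hub button for authority only.
; It also updates the HUD ranking, swaps Enhanced Input mapping contexts and relays mascot lines.
; Quest-item highlighting uses a Material Parameter Collection, a retriggerable delay and a timeline fade.
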(event `self.OpenCloseMenuOptions`
  (params (Value :type "InputActionValue Structure (by ref)"))
  (`/Engine/EditorBlueprintResources/StandardMacros.FlipFlop`
    (:`A`
      (`WidgetBlueprintLibrary.SetInputMode_GameAndUIEx` self null)
      (set `PlayerController.bShowMouseCursor` true))
    (:`B`
      (`WidgetBlueprintLibrary.SetInputMode_GameOnly` self)
      (set `PlayerController.bShowMouseCursor` false))))

(event `self.OnPlayerDead`
  (bind _death_restart (`self.Death_Restart`))
  ;[0 0 0] SHOW DEATH WIDGET
  (`KismetSystemLibrary.Delay` 3.5)
  (if (`self.IsLocalController`)
    (if (== _death_restart null)
      (bind _returnvalue (`|CreateWidget` "/Game/Blueprints/Widgets/WBP_DeathRestart.WBP_DeathRestart_C" null (cast `/Game/Blueprints/Characters/BP_PrisonnerDD` (`self.K2_GetPawn`) :!pure true)))
      (bind _output_get (set `self.Death_Restart` _returnvalue))
      (`UserWidget.AddToViewport` _output_get 0)
      (`/Game/Blueprints/Widgets/WBP_DeathRestart.ShowDeathWidget` (`self.Death_Restart`))
      (else
        (`UserWidget.AddToViewport` _death_restart 0)
        (`/Game/Blueprints/Widgets/WBP_DeathRestart.ShowDeathWidget` (`self.Death_Restart`))))))

(event `self.PrintWinner`
  (params (WithSuccess :type Boolean))
  ;[0 0 0] LEADERBOARDS WIDGET
  (bind _returnvalue (`|CreateWidget` "/Game/Blueprints/Widgets/WBP_EndGameWidget.WBP_EndGameWidget_C" null WithSuccess))
  (bind _output_get (set `self.EndGameWidget` _returnvalue))
  (`UserWidget.AddToViewport` _output_get 0)
  (if WithSuccess
    (`/Game/Blueprints/Widgets/WBP_EndGameWidget.RefreshLeaderboard` _output_get (`OnlineGameState.Leaderboard` (cast `OnlineGameState` (`GameplayStatics.GetGameState`) :!pure true)))
    (`/Game/Blueprints/Widgets/WBP_EndGameWidget.PrintWinner` (`self.EndGameWidget`) (`self.WinnerName`)))
  (`/Engine/EditorBlueprintResources/ActorMacros.Switch Has Authority`
    (:`Authority`
      (bind _endgamewidget (`self.EndGameWidget`)
        (:`then`
          (`Widget.SetVisibility` (`/Game/Blueprints/Widgets/WBP_EndGameWidget.ButtonBackToHub` _endgamewidget) "Visible"))
        (:`else`)))))

(event `self.OnPlayerRespawn`
  ;[0 0 0] REMOVE DEATH WIDGET WHEN RESPAWN
  (if (`self.IsLocalController`)
    (`|ExecutionSequence`
      (:`then_0`
        (bind _death_restart (`self.Death_Restart`)
          (:`then`
            (`Widget.RemoveFromParent` _death_restart))
          (:`else`)))
      (:`then_1`
        (`/Game/Blueprints/Characters/BP_PrisonnerDD.Respawn_Effect` (cast `/Game/Blueprints/Characters/BP_PrisonnerDD` (`self.K2_GetPawn`) :!pure true))))))

(event `MascotPrintOnClient`
  (params (TextToPrint :type "Array of String") (NewParam :type "/Game/Blueprints/Characters/BP_PrisonerController Object Reference"))
  (`self.Printer` NewParam TextToPrint))

(event `Printer`
  (params (Array :type "Array of String"))
  (for _array_element Array
    (`MascotAvatar.PrintLineAlone` (`self.MascotAvatar`) _array_element false)))

(event `self.HollowQuestItems`
  (`KismetMaterialLibrary.SetScalarParameterValue` (`self.MaterialToHollow`) (`self.Parameter Name`) 0.5)
  (`KismetSystemLibrary.RetriggerableDelay` 5.0)
  (bind (_direction _highlight) (`Timeline|Fade`)
    (:`Update`
      (`KismetMaterialLibrary.SetScalarParameterValue` (`self.MaterialToHollow`) (`self.Parameter Name`) _highlight))))

(event `self.BP_OnLeaderboardChanged`
  (params (Leaderboard :type "Array of PlayerScore Structure (by ref)"))
  (`/Game/Blueprints/Widgets/WBP_Leaderboard.UpdateRanking` (`/Game/Blueprints/Widgets/WBP_HUD.WBP_Leaderboard` (`/Game/Blueprints/Widgets/WBP_InGameWidget.WBP_HUD` (`self.UI`))) Leaderboard))

(event `SwitchInteractionMapping`
  (params (Default_IMC :type "InputMappingContext Object Reference") (New_IMC :type "InputMappingContext Object Reference"))
  (bind _returnvalue (subsystem `EnhancedInputLocalPlayerSubsystem`))
  (`EnhancedInputSubsystemInterface.RemoveMappingContext` _returnvalue Default_IMC (struct))
  (`EnhancedInputSubsystemInterface.AddMappingContext` _returnvalue New_IMC 0 (struct)))

(event `EnhancedInput|/Game/Blueprints/Inputs/Actions/IA_Interact`
  (params (ActionValue :type Boolean) (ElapsedSeconds :type "Float (double-precision)") (TriggeredSeconds :type "Float (double-precision)") (InputAction :type "InputAction Object Reference" :default "/Game/Blueprints/Inputs/Actions/IA_Interact.IA_Interact")))

(event `OnPlayerInteract`)

(fn `GetMascotAvatar`
  (returns (ReturnValue :type "MascotAvatar Object Reference"))
  (return (`self.MascotAvatar`)))

(fn `UserConstructionScript`)