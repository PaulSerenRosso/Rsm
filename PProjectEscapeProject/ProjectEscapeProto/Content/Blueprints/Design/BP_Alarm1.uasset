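; BP_Alarm1 is an interactable alarm button, prompted as an instant "Press" to "activate alarm mode", that is largely a stub.
; It implements interaction functions: CanInteract always allows use, while IsInteractionValid always returns false and TryInteract has no logic.
; Event_MulticastMoveDoor forwards to ButtonPress, which is empty, so no alarm behavior is implemented here.
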(event `Event_MulticastMoveDoor`
  (`self.ButtonPress`))

(event `ButtonPress`)

(fn `CanInteract`
  (params (Actor :type "Actor Object Reference"))
  (returns (ReturnValue :type Boolean))
  (return true))

(fn `GetInteractionHoldTime`
  (returns (ReturnValue :type "Float (single-precision)"))
  (return 0.0))

(fn `GetInteractionName`
  (returns (ReturnValue :type String))
  (return "activate alarm mode"))

(fn `GetTypeInteractionName`
  (returns (ReturnValue :type String))
  (return "Press "))

(fn `IsInteractionValid`
  (params (Actor :type "Actor Object Reference"))
  (returns (ReturnValue :type Boolean))
  (return false))

(fn `TryInteract`
  (params (Actor :type "Actor Object Reference"))
  (returns (ReturnValue :type Boolean)))

(fn `TryStopInteract`
  (params (Actor :type "Actor Object Reference"))
  (returns (ReturnValue :type Boolean))
  (return false))

(fn `UserConstructionScript`)