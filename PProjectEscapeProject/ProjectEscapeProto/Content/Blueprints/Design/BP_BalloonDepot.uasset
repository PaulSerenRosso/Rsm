(event `self.ReceiveBeginPlay`
  ;[0 0 0] Initialize Dyn Mat
  (`KismetSystemLibrary.Delay` 0.2)
  (bind _aswbp_interactable (cast `/Game/Blueprints/Widgets/WBP_Interactable` (`WidgetComponent.GetWidget` (`self.InteractionWidget`))))
  (bind _output_get (set `self.As WBP Interactable` _aswbp_interactable))
  (`Border.SetBrushFromMaterial` (`/Game/Blueprints/Widgets/WBP_Interactable.SlotUI` _output_get) (`self.MaterialInstance`)))

(event `self.BP_OnBalloonFinished`
  (params (WithSuccess :type Boolean))
  (if WithSuccess
    (`self.SwitchOffPreviz`)
    (`GameplayStatics.PlaySound2D` "/Game/Sounds/SoundWave/A_PlasticSqueak.A_PlasticSqueak" 1.0 1.0 0.0 null null)))

(event `self.BP_OnCannotInteract`
  (bind _as_wbp_interactable (`self.As WBP Interactable`))
  ;[0 0 0] POP UP
  (set `Border.ContentColorAndOpacity` (struct :`R` 0.395833 :`G` 0.395833 :`B` 0.395833 :`A` 0.5) (`/Game/Blueprints/Widgets/WBP_Interactable.SlotUI` _as_wbp_interactable))
  (set `TextBlock.Text` (`KismetTextLibrary.Conv_StringToText` (`KismetStringLibrary.Concat_StrStr` "You need " (`self.InteractableName`))) (`/Game/Blueprints/Widgets/WBP_Interactable.InteractionText` _as_wbp_interactable))
  (`SceneComponent.SetVisibility` (`self.InteractionWidget`) true false))

(event `self.BP_OnBalloonStarted`)

(event `self.UpdateBalloonDepotUI`
  (params (BalloonPercent :type "Float (single-precision)")))

(event `SwitchOffPreviz`
  (`PrimitiveComponent.SetMaterial` (`self.Sphere`) 0 "/Game/StarterContent/Materials/MI_Balloon.MI_Balloon"))

(fn `UserConstructionScript`
  (`SceneComponent.K2_AttachToComponent` (`self.InteractionRoot`) (`self.ItemMesh`) "None" "KeepRelative" "KeepRelative" "KeepRelative" true)
  (`SceneComponent.K2_AttachToComponent` (`self.InteractionSphere`) (`self.InteractionRoot`) "None" "KeepRelative" "KeepRelative" "KeepRelative" true))