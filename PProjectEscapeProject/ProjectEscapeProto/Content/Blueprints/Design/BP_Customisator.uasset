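; Interactable customization station where a prisoner picks an outfit color, previewed on its own skeletal mesh.
; Interaction multicasts, but only the locally controlled player gets the color picker, cursor and interactible input mapping; IA_Interact reverses this.
; Color changes go through the pawn's server event and delayed client apply, then tint the station's upper and lower body dynamic materials for the local caster.
; Delayed IsInteracting updates gate exit and re-interaction.
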(event `self.ReceiveBeginPlay`
  ;[0 0 0] BEGIN PLAY
  (bind _asbp_prisonner_dd (cast `/Game/Blueprints/Characters/BP_PrisonnerDD` (`Controller.K2_GetPawn` (`GameplayStatics.GetPlayerController` 0))))
  (set `self.As BP Prisonner DD` _asbp_prisonner_dd)
  (bind _returnvalue (`|CreateWidget` "/Game/Blueprints/Widgets/WBP_ColorPicker.WBP_ColorPicker_C" null _asbp_prisonner_dd))
  (set `self.Widget` _returnvalue)
  (add `self.OnInteract` (delegate `Event_OnInteract`))
  (add `/Game/Blueprints/Widgets/WBP_ColorPicker.OnColorChanged` (`self.Widget`) (delegate `Event_OnColorChanged`))
  ;[0 0 0] CREATE MID
  (bind _returnvalue_2 (`KismetMaterialLibrary.CreateDynamicMaterialInstance` "/Game/Art/Characters/CharacterPlayer/Materials/MI_UpperBody_map.MI_UpperBody_map"))
  (set `self.UpperMat` _returnvalue_2)
  (bind _returnvalue_3 (`KismetMaterialLibrary.CreateDynamicMaterialInstance` "/Game/Art/Characters/CharacterPlayer/Materials/MI_LowerBody_map.MI_LowerBody_map"))
  (set `self.LowerMat` _returnvalue_3)
  (`PrimitiveComponent.SetMaterial` (`self.SkeletalMesh`) 2 (`self.UpperMat`))
  (`PrimitiveComponent.SetMaterial` (`self.SkeletalMesh`) 0 (`self.LowerMat`)))

(event `Event_OnColorChanged`
  (params (Caster :type "Pawn Object Reference"))
  (bind _selectedcolora (`/Game/Blueprints/Widgets/WBP_ColorPicker.SelectedColorA` (`self.Widget`)))
  ;[0 0 0] CREATE MID
  (`/Game/Blueprints/Characters/BP_PrisonnerDD.Server_EventColorPick` (`self.As BP Prisonner DD`) _selectedcolora)
  (`KismetSystemLibrary.Delay` 0.2)
  (`/Game/Blueprints/Characters/BP_PrisonnerDD.Client_ApplyColorFromInstance` (`self.As BP Prisonner DD`) false)
  (if (`Pawn.IsLocallyControlled` Caster)
    (`MaterialInstanceDynamic.SetVectorParameterValue` (`self.UpperMat`) "ColorDetail" _selectedcolora)
    (`MaterialInstanceDynamic.SetVectorParameterValue` (`self.LowerMat`) "ColorDetail" _selectedcolora)))

(event `Event_OnInteract` :!signature `self.OnInteract`
  (params (Prisoner :type "Prisoner Object Reference"))
  ;[0 0 0] ENTER
  (`self.Multicast_Interact` Prisoner))

(event `Multicast_Interact`
  (params (Target :type "Pawn Object Reference"))
  (bind _asbp_prisoner_controller (cast `/Game/Blueprints/Characters/BP_PrisonerController` (`Pawn.GetController` Target) :!pure true))
  (if (`Pawn.IsLocallyControlled` Target)
    (`UserWidget.AddToViewport` (`self.Widget`) 0)
    (`/Game/Blueprints/Characters/BP_PrisonerController.SwitchInteractionMapping` _asbp_prisoner_controller "/Game/Blueprints/Inputs/IMC_Default.IMC_Default" "/Game/Blueprints/Inputs/IMC_Interactible.IMC_Interactible")
    (`self.EnableInput` _asbp_prisoner_controller)
    (set `PlayerController.bShowMouseCursor` true _asbp_prisoner_controller)
    (`KismetSystemLibrary.Delay` 1.0)
    (set `self.IsInteracting` true)))

(event `EnhancedInput|/Game/Blueprints/Inputs/Actions/IA_Interact`
  (params (ActionValue :type Boolean) (ElapsedSeconds :type "Float (double-precision)") (TriggeredSeconds :type "Float (double-precision)") (InputAction :type "InputAction Object Reference" :default "/Game/Blueprints/Inputs/Actions/IA_Interact.IA_Interact"))
  (bind _returnvalue (`GameplayStatics.GetPlayerController` 0))
  ;[0 0 0] EXIT
  (:`Triggered`
    (if (`self.IsInteracting`)
      (`Widget.RemoveFromParent` (`self.Widget`))
      (`/Game/Blueprints/Characters/BP_PrisonerController.SwitchInteractionMapping` (cast `/Game/Blueprints/Characters/BP_PrisonerController` (`GameplayStatics.GetPlayerController` 0) :!pure true) "/Game/Blueprints/Inputs/IMC_Interactible.IMC_Interactible" "/Game/Blueprints/Inputs/IMC_Default.IMC_Default")
      (set `PlayerController.bShowMouseCursor` false _returnvalue)
      (`self.DisableInput` _returnvalue)
      (`KismetSystemLibrary.Delay` 0.2)
      (set `self.IsInteracting` false))))

(fn `CanInteract`
  (params (Actor :type "Actor Object Reference"))
  (returns (ReturnValue :type Boolean))
  (return (not (`self.IsInteracting`))))

(fn `UserConstructionScript`
  (`SceneComponent.K2_AttachToComponent` (`self.InteractionRoot`) (`self.ItemMesh`) "None" "KeepRelative" "KeepRelative" "KeepRelative" true)
  (`SceneComponent.K2_AttachToComponent` (`self.InteractionSphere`) (`self.InteractionRoot`) "None" "KeepRelative" "KeepRelative" "KeepRelative" true))