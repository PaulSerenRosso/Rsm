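; BP_Door_Tutorial is a two-panel door Blueprint that opens and closes through OpenDoors and CloseDoors events.
; OpenDoors plays a Timeline whose Alpha scales each door's goal vector into its relative location, and CloseDoors reverses that Timeline.
; Because positions are the scaled goals rather than offsets from starting transforms, an Alpha of zero puts both doors at their relative origin.
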(event `Open Doors`
  (bind (_direction _alpha) (`Timeline|Timeline` :!label _label)
    (:`Update`
      (`|ExecutionSequence`
        (:`then_0`
          (`SceneComponent.K2_SetRelativeLocation` (`self.Door1`) (* _alpha (`self.GoalDoor1`)) false false))
        (:`then_1`
          (`SceneComponent.K2_SetRelativeLocation` (`self.Door2`) (* _alpha (`self.GoalDoor2`)) false false))))))

(event `Close Doors`
  (goto _label :!via `Reverse`))

(fn `UserConstructionScript`)