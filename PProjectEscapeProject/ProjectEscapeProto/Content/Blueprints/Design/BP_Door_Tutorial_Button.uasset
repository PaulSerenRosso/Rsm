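; Tutorial door actor that a child-actor HUB button toggles between open and closed.
; The button's OnInteract event plays or reverses a Timeline that slides DoorLeft; the DoorRight update is disconnected.
; After a short delay for multiplayer, an IsMoving flag blocks presses mid-motion, and a dynamic material turns the button red until movement finishes.
; Two-panel OpenDoors and CloseDoors events using MoveComponentTo are not called within this graph.
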(event `self.ReceiveBeginPlay`
  (bind _asbp_button_interactable_hub (cast `/Game/Blueprints/Objects/BP_ButtonInteractableHUB` (`ChildActorComponent.ChildActor` (`self.Button`))))
  (add `InteractableObjects.OnInteract` _asbp_button_interactable_hub (delegate `Event_OnInteract`))
  (bind _returnvalue (`PrimitiveComponent.CreateDynamicMaterialInstance` (`/Game/Blueprints/Objects/BP_ButtonInteractableHUB.SM_Button_02` _asbp_button_interactable_hub) 0 null "None"))
  (set `self.Material Button` _returnvalue))

(event `Event_OnInteract`
  (`self.On Button Pressed`))

(event `On Button Pressed`
  (`KismetSystemLibrary.PrintString` "Hello")
  (`self.ButtonPress`)
  ;[0 0 0] CAN'T OPEN WHILE DOOR IS MOVING
  ;;[0 0 0] DELAY TO AVOID MULTIPLAYER PROBLEMS
  (`KismetSystemLibrary.Delay` 0.1)
  (if (not (`self.IsMoving`))
    (set `self.IsMoving` true)
    (`MaterialInstanceDynamic.SetVectorParameterValue` (`self.Material Button`) "EmissiveColor" (struct :`R` 0.854167 :`A` 1.0))
    ;[0 0 0] CHECK IF CLOSE
    (if (`self.Close`)
      (set `self.Close` false)
      ;[0 0 0] DOOR MOVEMENT
      (bind (_direction _alpha) (`Timeline|Timeline` :!label _label)
        (:`Update`
          (`|ExecutionSequence`
            (:`then_0`
              (`SceneComponent.K2_SetRelativeLocation` (`self.Door_Left`) (* _alpha (`self.Distance_Gauche`)) false false))))
        (:`Finished`
          (set `self.IsMoving` false)
          (`MaterialInstanceDynamic.SetVectorParameterValue` (`self.Material Button`) "EmissiveColor" (struct :`R` 1.0 :`G` 1.0 :`B` 1.0 :`A` 1.0))))
      (else
        (set `self.Close` true)
        (goto _label :!via `Reverse`)))))

(event `ButtonPress`
  (if (not (`self.IsPress`))
    (set `self.IsPress` true)))

(event `Open Doors`
  (bind _door_left (`self.Door_Left`))
  (bind _door_right (`self.Door_Right`))
  (`|ExecutionSequence`
    (:`then_0`
      (set `self.GoalDoor1` (+ (`SceneComponent.RelativeLocation` _door_left) (0.0 100.0 0.0)))
      (`KismetSystemLibrary.MoveComponentTo` _door_left (`self.GoalDoor1`) (struct) false false 2.0))
    (:`then_1`
      (set `self.GoalDoor2` (- (`SceneComponent.RelativeLocation` _door_right) (0.0 100.0 0.0)))
      (`KismetSystemLibrary.MoveComponentTo` _door_right (`self.GoalDoor2`) (struct) false false 2.0)))
  (`KismetSystemLibrary.PrintString` "END"))

(event `Close Doors`
  (bind _door_right (`self.Door_Right`))
  (bind _door_left (`self.Door_Left`))
  (`|ExecutionSequence`
    (:`then_0`
      (set `self.GoalDoor1` (- (`SceneComponent.RelativeLocation` _door_left) (0.0 100.0 0.0)))
      (`KismetSystemLibrary.MoveComponentTo` _door_left (`self.GoalDoor1`) (struct) false false 2.0))
    (:`then_1`
      (set `self.GoalDoor2` (+ (`SceneComponent.RelativeLocation` _door_right) (0.0 100.0 0.0)))
      (`KismetSystemLibrary.MoveComponentTo` _door_right (`self.GoalDoor2`) (struct) false false 2.0)))
  (`KismetSystemLibrary.PrintString` "END"))

(fn `UserConstructionScript`)