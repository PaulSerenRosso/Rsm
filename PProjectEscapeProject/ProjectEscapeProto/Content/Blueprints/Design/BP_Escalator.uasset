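; Escalator actor that carries an actor overlapping its steps along the mesh's forward vector and can be reversed from a bottom switch.
; A timeline started on overlap adds a relative offset scaled by ElevatorSpeed each update, plus an opposing offset once the overlap ends.
; Its interaction functions allow use at the switch, where a BP_PrisonnerDD triggers a multicast-named event that negates the speed.
; IsInteractionValid always returns false, and TryInteract prints debug text.
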(event `self.Steps.OnComponentBeginOverlap`
  (params (OverlappedComponent :type "PrimitiveComponent Object Reference") (OtherActor :type "Actor Object Reference") (OtherComp :type "PrimitiveComponent Object Reference") (OtherBodyIndex :type Integer) (bFromSweep :type Boolean) (SweepResult :type "HitResult Structure (by ref)"))
  (bind _rootcomponent (`Actor.RootComponent` OtherActor))
  (bind _returnvalue (* (`SceneComponent.GetForwardVector` (`self.SM_Escalator`)) (`self.ElevatorSpeed`)))
  (set `self.In Elevator` true)
  (bind (_direction _newtrack_0) (`Timeline|Timeline_0`)
    (:`Update`
      (`SceneComponent.K2_AddRelativeLocation` _rootcomponent (* _newtrack_0 _returnvalue) false false)
      (if (not (`self.In Elevator`))
        (`SceneComponent.K2_AddRelativeLocation` _rootcomponent (* (-1.0 -1.0 -1.0) _returnvalue) false false)))))

(event `self.Steps.OnComponentEndOverlap`
  (params (OverlappedComponent :type "PrimitiveComponent Object Reference") (OtherActor :type "Actor Object Reference") (OtherComp :type "PrimitiveComponent Object Reference") (OtherBodyIndex :type Integer))
  (set `self.In Elevator` false))

(event `self.Switch_Bottom.OnComponentBeginOverlap`
  (params (OverlappedComponent :type "PrimitiveComponent Object Reference") (OtherActor :type "Actor Object Reference") (OtherComp :type "PrimitiveComponent Object Reference") (OtherBodyIndex :type Integer) (bFromSweep :type Boolean) (SweepResult :type "HitResult Structure (by ref)"))
  (set `self.In Front Of Switch` true))

(event `self.Switch_Bottom.OnComponentEndOverlap`
  (params (OverlappedComponent :type "PrimitiveComponent Object Reference") (OtherActor :type "Actor Object Reference") (OtherComp :type "PrimitiveComponent Object Reference") (OtherBodyIndex :type Integer))
  (set `self.In Front Of Switch` false))

(event `Event_MultiCastEscalator`
  (set `self.ElevatorSpeed` (* (`self.ElevatorSpeed`) -1.0)))

(fn `CanInteract`
  (params (Actor :type "Actor Object Reference"))
  (returns (ReturnValue :type Boolean))
  (return (`self.In Front Of Switch`)))

(fn `GetInteractionHoldTime`
  (returns (ReturnValue :type "Float (single-precision)"))
  (return 0.0))

(fn `GetInteractionName`
  (returns (ReturnValue :type String))
  (return ""))

(fn `GetTypeInteractionName`
  (returns (ReturnValue :type String))
  (return ""))

(fn `IsInteractionValid`
  (params (Actor :type "Actor Object Reference"))
  (returns (ReturnValue :type Boolean))
  (return false))

(fn `TryInteract`
  (params (Actor :type "Actor Object Reference"))
  (returns (ReturnValue :type Boolean))
  (cast `/Game/Blueprints/Characters/BP_PrisonnerDD` Actor)
  (`KismetSystemLibrary.PrintString` "Hello")
  (`self.Event_MultiCastEscalator`)
  (return false))

(fn `TryStopInteract`
  (params (Actor :type "Actor Object Reference"))
  (returns (ReturnValue :type Boolean))
  (return false))

(fn `UserConstructionScript`)