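; BP_Escape triggers the level's escape alarm when the online game mode signals the last phase.
; It sets the "Escape" environment parameter, shows a fade-text widget, plays two staggered sirens and has the player's mascot announce time out and point to the central elevator.
; RedLight turns every spot, point and rect light red and swaps the material on meshes tagged SkyPanel.
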(event `self.ReceiveBeginPlay`
  (bind _asonline_game_mode (cast `OnlineGameMode` (`GameplayStatics.GetGameMode`)))
  (add `OnlineGameMode.IsLastPhasis` _asonline_game_mode (delegate `Event_LastPhasis`)))

(event `Event_LastPhasis`
  (`self.Widget`)
  (`self.RedLight`))

(event `Widget`
  (`KismetMaterialLibrary.SetScalarParameterValue` "/Game/Art/Environments/Materials/MPC_Environments.MPC_Environments" "Escape" 1.0)
  (bind _returnvalue (`|CreateWidget` "/Game/Blueprints/Widgets/Tutorial/BP_FadeTextEscape.BP_FadeTextEscape_C" (`GameplayStatics.GetPlayerController` 0)))
  (`UserWidget.AddToViewport` _returnvalue 0)
  (`GameplayStatics.PlaySound2D` "/Game/Sounds/SoundWave/A_Siren2.A_Siren2" 1.0 1.0 0.0 null null)
  (`self.RedLight`)
  (`KismetSystemLibrary.Delay` 0.5)
  (`GameplayStatics.PlaySound2D` "/Game/Sounds/SoundWave/A_Siren1.A_Siren1" 1.0 1.0 0.0 null null)
  (bind _asbp_prisonner_dd (cast `/Game/Blueprints/Characters/BP_PrisonnerDD` (`GameplayStatics.GetPlayerCharacter` 0)))
  (`/Game/Blueprints/Characters/BP_PrisonnerDD.PrintMascotLine` _asbp_prisonner_dd "Time out ! I suggest you go to the central part of the level and take the elevator, except if you want to die painfully !" false))

(event `RedLight`
  (`|ExecutionSequence`
    (:`then_0`
      (bind _outactors (`GameplayStatics.GetAllActorsOfClass` "/Script/Engine.SpotLight"))
      (for _array_element _outactors
        (`LightComponent.SetLightColor` (`Light.LightComponent` _array_element) (struct :`R` 1.0 :`G` 0.058993 :`A` 1.0) true)))
    (:`then_1`
      (bind _outactors_2 (`GameplayStatics.GetAllActorsOfClass` "/Script/Engine.PointLight"))
      (for _array_element_2 _outactors_2
        (`LightComponent.SetLightColor` (`Light.LightComponent` _array_element_2) (struct :`R` 1.0 :`G` 0.058993 :`A` 1.0) true)))
    (:`then_2`
      (bind _outactors_3 (`GameplayStatics.GetAllActorsOfClass` "/Script/Engine.RectLight"))
      (for _array_element_3 _outactors_3
        (`LightComponent.SetLightColor` (`Light.LightComponent` _array_element_3) (struct :`R` 1.0 :`G` 0.058993 :`A` 1.0) true)))
    (:`then_3`
      (bind _outactors_4 (`GameplayStatics.GetAllActorsOfClassWithTag` "/Script/Engine.StaticMeshActor" "SkyPanel"))
      (for _array_element_4 _outactors_4
        (`PrimitiveComponent.SetMaterial` (`StaticMeshActor.StaticMeshComponent` _array_element_4) 0 "/Game/Art/Environments/Materials/MaterialInstances/MI_RoofDistrict_04.MI_RoofDistrict_04")))))

(event `self.ReceiveEndPlay`
  (params (EndPlayReason :type "EEndPlayReason Enum" :default "Destroyed")))

(fn `UserConstructionScript`)