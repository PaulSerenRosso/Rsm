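; BP_ItemDispenser is an interactable vending-machine-style distributor that spawns a configurable item, apparently a trap, at its spawn point.
; Interacting while it is ready spawns the item and locks the machine for a delivery cooldown.
; Multicast events switch the dynamic material's emissive between red and white, swap the loading and ready sounds, toggle availability, and play a completion sound when ready again.
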(event `UpdateDistributorDataGreen_MULTICAST`
  (bind _materialdistrib (`self.MaterialDistrib`))
  ;[0 0 0] Réplication Couleur
  (`MaterialInstanceDynamic.SetVectorParameterValue` _materialdistrib "EmissiveMultiplyColor" (struct :`R` 1.0 :`G` 1.0 :`B` 1.0 :`A` 1.0))
  (`MaterialInstanceDynamic.SetScalarParameterValue` _materialdistrib "EmissiveInt" 0.5)
  (`GameplayStatics.PlaySoundAtLocation` "/Game/Sounds/SoundCue/A_TaskCompleted.A_TaskCompleted" (`SceneComponent.K2_GetComponentLocation` (`self.Distributor`)) (struct) 1.0 1.0 0.0 null null null null)
  (`AudioComponent.SetSound` (`self.A_SFX_Distributor`) "/Game/Sounds/SoundCue/SFX/Environments/A_SFX_Distributor.A_SFX_Distributor")
  (set `self.CanSpawnTrap` true))

(event `UpdateDistributorDataRed_Multicast`
  (bind _materialdistrib (`self.MaterialDistrib`))
  ;[0 0 0] Réplication couleur
  (`MaterialInstanceDynamic.SetVectorParameterValue` _materialdistrib "EmissiveMultiplyColor" (struct :`R` 1.0 :`G` 0.016606 :`A` 1.0))
  (`MaterialInstanceDynamic.SetScalarParameterValue` _materialdistrib "EmissiveInt" 0.1)
  (`AudioComponent.SetSound` (`self.A_SFX_Distributor`) "/Game/Sounds/SoundCue/SFX/Environments/A_SFX_DistributorLoading.A_SFX_DistributorLoading")
  (set `self.CanSpawnTrap` false))

(event `self.ReceiveBeginPlay`
  (add `self.OnInteract` (delegate `SpawnTrap`))
  (bind _returnvalue (`PrimitiveComponent.CreateDynamicMaterialInstance` (`self.Distributor`) 0 "/Game/Art/Environments/Materials/MaterialInstances/Props/MI_VendingMachine.MI_VendingMachine" "None"))
  (set `self.MaterialDistrib` _returnvalue))

(event `SpawnTrap` :!signature `self.OnInteract`
  (params (Prisoner :type "Prisoner Object Reference"))
  (if (`self.CanSpawnTrap`)
    (`self.UpdateDistributorDataRed_Multicast`)
    (`|SpawnActorFromClass` (`self.ItemToSpawn`) (`SceneComponent.K2_GetComponentToWorld` (`self.SpawnPoint`)) "Undefined" "MultiplyWithRoot" null null)
    (`KismetSystemLibrary.Delay` (`self.DeliverCooldown`))
    (`self.UpdateDistributorDataGreen_MULTICAST`)))

(fn `GetInteractionName`
  (returns (ReturnValue :type String))
  (return ""))

(fn `UserConstructionScript`
  (bind _interactionroot (`self.InteractionRoot`))
  (`SceneComponent.K2_AttachToComponent` _interactionroot (`self.ItemMesh`) "None" "KeepRelative" "KeepRelative" "KeepRelative" true)
  (`SceneComponent.K2_AttachToComponent` (`self.InteractionSphere`) _interactionroot "None" "KeepRelative" "KeepRelative" "KeepRelative" true)
  (`SceneComponent.K2_AttachToComponent` (`self.InteractionWidget`) _interactionroot "None" "KeepRelative" "KeepRelative" "KeepRelative" true))