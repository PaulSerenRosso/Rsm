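; BP_Mirror is an interactable mirror that opens and closes a color picker widget.
; On BeginPlay it binds SpawnTrap to OnInteract; despite its name, that event only toggles the UI through the IsWidgetVisible flag.
; Opening creates a new WBP_ColorPicker, shows the mouse cursor and disables player controller input, while closing removes the widget and reverts both.
; GetInteractionName returns an empty string.
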(event `self.ReceiveBeginPlay`
  (add `self.OnInteract` (delegate `SpawnTrap`)))

(event `SpawnTrap`
  (bind _returnvalue (`GameplayStatics.GetPlayerController` 0))
  (if (`self.IsWidgetVisible`)
    (`Widget.RemoveFromParent` (stale _returnvalue_2))
    (set `PlayerController.bShowMouseCursor` false _returnvalue)
    (`self.EnableInput` _returnvalue null)
    (set `self.IsWidgetVisible` false)
    (else
      (bind _returnvalue_2 (`|CreateWidget` "/Game/Blueprints/Widgets/WBP_ColorPicker.WBP_ColorPicker_C"))
      (`UserWidget.AddToViewport` _returnvalue_2 0)
      (set `PlayerController.bShowMouseCursor` true _returnvalue)
      (`self.DisableInput` _returnvalue null)
      (set `self.IsWidgetVisible` true))))

(fn `GetInteractionName`
  (returns (ReturnValue :type String))
  (return ""))

(fn `UserConstructionScript`)