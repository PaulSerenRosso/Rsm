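; BP_Screen is an interactable screen actor set up for multiplayer, with most of its logic still unfinished or disconnected.
; On BeginPlay it binds to an OnInteract event that forwards to a multicast event, whose branch does nothing.
; InteractionSphere overlap events are empty, while the debug-printed interacting-player counter sits unwired.
; RepNotify functions for screens, player count and the two-player flag are empty stubs.
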(event `self.ReceiveBeginPlay`
  ;[1 1 1] Réplication
  (add `self.OnInteract` (delegate `OnInteract_Event`)))

(event `OnInteract_Event`
  ;[1 1 1] Réplication
  (`self.EventMulticast`))

(event `EventMulticast`
  (if true
    _))

(event `self.InteractionSphere.OnComponentBeginOverlap`
  (params (OverlappedComponent :type "PrimitiveComponent Object Reference") (OtherActor :type "Actor Object Reference") (OtherComp :type "PrimitiveComponent Object Reference") (OtherBodyIndex :type Integer) (bFromSweep :type Boolean) (SweepResult :type "HitResult Structure (by ref)"))
  ;[1 1 1] Check du nombre de joueurs
)

(event `self.InteractionSphere.OnComponentEndOverlap`
  (params (OverlappedComponent :type "PrimitiveComponent Object Reference") (OtherActor :type "Actor Object Reference") (OtherComp :type "PrimitiveComponent Object Reference") (OtherBodyIndex :type Integer))
  ;[1 1 1] Check du nombre de joueurs
)

(fn `OnRep_2PlayersInteracting?`)

(fn `OnRep_PlayerInteracting`)

(fn `OnRep_Screens`)

(fn `UserConstructionScript`)