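; Elevator actor with two sliding doors, driven by multicast events to open, close or snap shut.
; On BeginPlay it caches both door positions, then open and close timelines feed UpdateDoorsPosition to offset the doors in opposite directions along local Y.
; Opened and closed notifications fire when the motion completes; the waiting-time events are empty, and the emissive material, prisoner and voice logic is disconnected.
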(event `self.ReceiveBeginPlay`
  (set `self.LeftDoorPos` (`SceneComponent.RelativeLocation` (`self.Door_Left`)))
  (set `self.RightDoorPos` (`SceneComponent.RelativeLocation` (`self.Door_Right`))))

(event `self.BP_Server_StartWaitingTime`)

(event `self.BP_Multicast_StopWaitingTime`)

(event `self.BP_Multicast_CloseImmediately`
  (`SceneComponent.K2_SetRelativeLocation` (`self.Door_Left`) (`self.LeftDoorPos`) false false)
  (`SceneComponent.K2_SetRelativeLocation` (`self.Door_Right`) (`self.RightDoorPos`) false false)
  (`self.OnElevatorClosed`))

(event `self.BP_Multicast_OpenElevator`
  (bind (_direction _alpha) (`Timeline|OpenDoors` :!via `PlayFromStart`)
    (:`Update`
      (`self.UpdateDoorsPosition` _alpha))
    (:`Finished`
      (`self.OnElevatorOpened`))))

(event `self.BP_Multicast_CloseElevator`
  (bind (_direction _alpha) (`Timeline|CloseDoor` :!via `PlayFromStart`)
    (:`Update`
      (`self.UpdateDoorsPosition` _alpha))
    (:`Finished`
      (`self.OnElevatorClosed`))))

(fn `UpdateDoorsPosition`
  (params (Distance :type "Float (double-precision)"))
  (bind (_leftdoorpos_x _leftdoorpos_y _leftdoorpos_z) (`KismetMathLibrary.BreakVector` (`self.LeftDoorPos`)))
  (bind (_rightdoorpos_x _rightdoorpos_y _rightdoorpos_z) (`KismetMathLibrary.BreakVector` (`self.RightDoorPos`)))
  (bind _returnvalue (* Distance (`self.DistanceDoor`)))
  (`SceneComponent.K2_SetRelativeLocation` (`self.Door_Left`) (`KismetMathLibrary.MakeVector` _leftdoorpos_x (- _leftdoorpos_y _returnvalue) _leftdoorpos_z) false false)
  (`SceneComponent.K2_SetRelativeLocation` (`self.Door_Right`) (`KismetMathLibrary.MakeVector` _rightdoorpos_x (+ _rightdoorpos_y _returnvalue) _rightdoorpos_z) false false))

(fn `UserConstructionScript`)