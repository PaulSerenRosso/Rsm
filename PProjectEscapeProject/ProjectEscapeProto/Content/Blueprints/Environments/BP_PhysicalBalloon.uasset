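; BP_PhysicalBalloon is an environment actor with four balloon components that are pushed upward through physics.
; On BeginPlay it applies random linear damping to the balloons and a first upward acceleration force.
; A looping timer then calls EventBalloonForce to reapply that force at short intervals, simulating lift with periodic pushes rather than on Tick.
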(event `self.ReceiveBeginPlay`
  (`PrimitiveComponent.SetLinearDamping` (`self.Balloon`) (`KismetMathLibrary.RandomFloat`))
  (`PrimitiveComponent.SetLinearDamping` (`self.Balloon1`) (`KismetMathLibrary.RandomFloat`))
  (`PrimitiveComponent.SetLinearDamping` (`self.Balloon2`) (`KismetMathLibrary.RandomFloat`))
  (`PrimitiveComponent.SetLinearDamping` (`self.Balloon3`) (`KismetMathLibrary.RandomFloat`))
  (`PrimitiveComponent.AddForce` (`self.Balloon`) (0.0 0.0 500.0) "None" true)
  (`PrimitiveComponent.AddForce` (`self.Balloon1`) (0.0 0.0 500.0) "None" true)
  (`PrimitiveComponent.AddForce` (`self.Balloon2`) (0.0 0.0 500.0) "None" true)
  (`PrimitiveComponent.AddForce` (`self.Balloon3`) (0.0 0.0 500.0) "None" true)
  (`KismetSystemLibrary.K2_SetTimer` null "EventBalloonForce" 0.1 true true))

(event `EventBalloonForce`
  (`PrimitiveComponent.AddForce` (`self.Balloon`) (0.0 0.0 500.0) "None" true)
  (`PrimitiveComponent.AddForce` (`self.Balloon1`) (0.0 0.0 500.0) "None" true)
  (`PrimitiveComponent.AddForce` (`self.Balloon2`) (0.0 0.0 500.0) "None" true)
  (`PrimitiveComponent.AddForce` (`self.Balloon3`) (0.0 0.0 500.0) "None" true))

(fn `UserConstructionScript`)