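; BP_SuburdsScreen is an environment screen that fades up its emissive glow the first time a BP_PrisonnerDD enters its trigger box.
; BeginPlay creates a dynamic instance of MI_RoofDistrict_01 on the Screen component and zeroes its EmissivePower parameter.
; The first valid Box overlap sets a one-shot flag and plays the Fade timeline, which drives a different parameter, EmissiveInt, with the scaled curve value.
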(event `self.ReceiveBeginPlay`
  (bind _returnvalue (`PrimitiveComponent.CreateDynamicMaterialInstance` (`self.Screen`) 0 "/Game/Art/Environments/Materials/MaterialInstances/MI_RoofDistrict_01.MI_RoofDistrict_01" "None"))
  (bind _output_get (set `self.MatScreen` _returnvalue))
  (`MaterialInstanceDynamic.SetScalarParameterValue` _output_get "EmissivePower" 0.0))

(event `self.Box.OnComponentBeginOverlap`
  (params (OverlappedComponent :type "PrimitiveComponent Object Reference") (OtherActor :type "Actor Object Reference") (OtherComp :type "PrimitiveComponent Object Reference") (OtherBodyIndex :type Integer) (bFromSweep :type Boolean) (SweepResult :type "HitResult Structure (by ref)"))
  (if (not (`self.HasOverlapped`))
    (bind _asbp_prisonner_dd (cast `/Game/Blueprints/Characters/BP_PrisonnerDD` OtherActor))
    (`/Engine/EditorBlueprintResources/StandardMacros.IsValid` _asbp_prisonner_dd
      (:`Is Valid`
        (set `self.HasOverlapped` true)
        (bind (_direction _fade) (`Timeline|Fade`)
          (:`Update`
            (`MaterialInstanceDynamic.SetScalarParameterValue` (`self.MatScreen`) "EmissiveInt" (* _fade 2.0))))))))

(fn `UserConstructionScript`)