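; Screen actor that displays a widget component's render target on a configurable static mesh.
; Construction applies the mesh, creates a dynamic instance of the chosen material on one slot and feeds it the widget texture.
; From BeginPlay, a looping timer reassigns that render target to the material ten times a second.
; A Fade event waits briefly, then plays a timeline that drives a named material parameter, scaled by the target value.
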(event `Fade`
  (params (TargetValue :type "Float (double-precision)"))
  (`KismetSystemLibrary.Delay` 0.5)
  (bind (_direction _fade) (`Timeline|Crank`)
    (:`Update`
      (`MaterialInstanceDynamic.SetScalarParameterValue` (`self.MID`) (`self.FadeParameterName`) (* _fade TargetValue)))))

(event `self.ReceiveBeginPlay`
  (`KismetSystemLibrary.K2_SetTimer` null "SetRenderTarget" 0.1 true))

(fn `SetRenderTarget`
  (`MaterialInstanceDynamic.SetTextureParameterValue` (`self.MID`) "Texture" (`WidgetComponent.GetRenderTarget` (`self.Widget`))))

(fn `UserConstructionScript`
  (`StaticMeshComponent.SetStaticMesh` (`self.StaticMesh`) (`self.Mesh`))
  (bind _returnvalue (`KismetMaterialLibrary.CreateDynamicMaterialInstance` (`self.Material`)))
  (set `self.MID` _returnvalue)
  (`PrimitiveComponent.SetMaterial` (`self.StaticMesh`) (`self.Element Index`) (`self.MID`))
  (`MaterialInstanceDynamic.SetTextureParameterValue` (`self.MID`) "Texture" (`WidgetComponent.GetRenderTarget` (`self.Widget`))))