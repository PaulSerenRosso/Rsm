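; Multiplayer sliding door toggled by two child button actors, with a multicast event driving a Timeline that moves the mesh.
; A shared dynamic material turns both buttons red during movement, and presses while moving only play a click.
; A server-side trigger box makes AI characters pause and open closed doors.
; If PlayerNeeded is set, buttons stay disabled until enough prisoners overlap the box, which unlocks and toggles this and linked doors.
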(event `self.ReceiveBeginPlay`
  (if (> (`self.PlayerNeeded`) 0)
    (`self.Switch Interaction Button` false))
  (bind _asbp_button_interactable (cast `/Game/Blueprints/Objects/BP_ButtonInteractable` (`ChildActorComponent.ChildActor` (`self.BP_Button_02`))))
  (bind _asbp_button_interactable_2 (cast `/Game/Blueprints/Objects/BP_ButtonInteractable` (`ChildActorComponent.ChildActor` (`self.BP_Button_01`))))
  (add `InteractableObjects.OnInteract` _asbp_button_interactable (delegate `Event_OnInteract`))
  (add `InteractableObjects.OnInteract` _asbp_button_interactable_2 (delegate `Event_OnInteract`))
  (set `/Game/Blueprints/Objects/BP_ButtonInteractable.RoomsAssimilited` (`self.Rooms Assimilited`) _asbp_button_interactable_2)
  (set `/Game/Blueprints/Objects/BP_ButtonInteractable.RoomsAssimilited` (`self.Rooms Assimilited`) _asbp_button_interactable)
  (bind _returnvalue (`PrimitiveComponent.CreateDynamicMaterialInstance` (`/Game/Blueprints/Objects/BP_ButtonInteractable.Mesh_Button` _asbp_button_interactable_2) 0 "/Game/Art/Environments/Materials/MaterialInstances/Props/MI_Buton.MI_Buton" "None"))
  (`PrimitiveComponent.SetMaterial` (`/Game/Blueprints/Objects/BP_ButtonInteractable.Mesh_Button` _asbp_button_interactable) 0 _returnvalue)
  (set `self.MaterialButton` _returnvalue)
  (`MaterialInstanceDynamic.SetVectorParameterValue` (`self.MaterialButton`) "EmissiveColor" (struct :`R` 1.0 :`G` 1.0 :`B` 1.0 :`A` 1.0)))

(event `Event_OnInteract`
  (params (Prisoner :type "Prisoner Object Reference"))
  (`self.Event_Multicast_OnButtonPressed`))

(event `Event_Multicast_OnButtonPressed`
  (bind _returnvalue (`SceneComponent.K2_GetComponentLocation` (`self.Door_Mesh`)))
  (`self.ButtonPress`)
  ;[0 0 0] CAN'T OPEN WHILE DOOR IS MOVING
  ;;[0 0 0] DELAY TO AVOID MULTIPLAYER PROBLEMS
  (`KismetSystemLibrary.Delay` 0.1)
  (if (`self.IsMoving`)
    (`GameplayStatics.PlaySoundAtLocation` "/Game/Sounds/SoundCue/UI/A_UI_Click.A_UI_Click" _returnvalue (struct) 1.0 1.0 0.0 null null null null)
    (else
      (set `self.IsMoving` true)
      (`GameplayStatics.PlaySoundAtLocation` "/Game/Sounds/SoundCue/UI/A_UI_AddPlayer.A_UI_AddPlayer" _returnvalue (struct) 1.0 1.0 0.0 null null null null)
      (`MaterialInstanceDynamic.SetVectorParameterValue` (`self.MaterialButton`) "EmissiveColor" (struct :`R` 0.854167 :`A` 1.0))
      ;[0 0 0] CHECK IF CLOSE
      (if (`self.Close`)
        (set `self.Close` false)
        ;[0 0 0] DOOR MOVEMENT
        (bind (_direction _alpha) (`Timeline|Timeline` :!label _label)
          (:`Update`
            (`SceneComponent.K2_SetRelativeLocation` (`self.Door_Mesh`) (* _alpha (`self.Distance`)) false false))
          (:`Finished`
            (set `self.IsMoving` false)
            (`MaterialInstanceDynamic.SetVectorParameterValue` (`self.MaterialButton`) "EmissiveColor" (struct :`R` 1.0 :`G` 1.0 :`B` 1.0 :`A` 1.0))))
        (else
          (set `self.Close` true)
          (goto _label :!via `Reverse`))))))

(event `ButtonPress`
  (if (not (`self.IsPress`))
    (set `self.IsPress` true)))

(event `self.Box.OnComponentBeginOverlap`
  (params (OverlappedComponent :type "PrimitiveComponent Object Reference") (OtherActor :type "Actor Object Reference") (OtherComp :type "PrimitiveComponent Object Reference") (OtherBodyIndex :type Integer) (bFromSweep :type Boolean) (SweepResult :type "HitResult Structure (by ref)"))
  (bind _playersinteracting (`self.PlayersInteracting`))
  (bind _doorslinked (`self.DoorsLinked`))
  (`/Engine/EditorBlueprintResources/ActorMacros.Switch Has Authority`
    (:`Authority`
      (bind _asaicharacter (cast `AICharacter` OtherActor)
        (:`then`
          (if (`self.Close`)
            (`AICharacter.SetWaitingTime` _asaicharacter 2.1)
            (`self.Event_Multicast_OnButtonPressed`)))
        (:`CastFailed`
          (if (> (`self.PlayerNeeded`) 0)
            (bind _asbp_prisonner_dd (cast `/Game/Blueprints/Characters/BP_PrisonnerDD` OtherActor))
            (`KismetArrayLibrary.Array_AddUnique` _playersinteracting (`PlayerState.PlayerId` (`Pawn.PlayerState` _asbp_prisonner_dd)))
            (if (not (> (`self.PlayerNeeded`) (`KismetArrayLibrary.Array_Length` _playersinteracting)))
              (`KismetArrayLibrary.Array_Add` _doorslinked self)
              (for _array_element _doorslinked
                (`self.Open Door with Num Players` _array_element)))))))))

(event `self.Box.OnComponentEndOverlap`
  (params (OverlappedComponent :type "PrimitiveComponent Object Reference") (OtherActor :type "Actor Object Reference") (OtherComp :type "PrimitiveComponent Object Reference") (OtherBodyIndex :type Integer))
  (`/Engine/EditorBlueprintResources/ActorMacros.Switch Has Authority`
    (:`Authority`
      (if (> (`self.PlayerNeeded`) 0)
        (bind _asbp_prisonner_dd (cast `/Game/Blueprints/Characters/BP_PrisonnerDD` OtherActor))
        (`KismetArrayLibrary.Array_RemoveItem` (`self.PlayersInteracting`) (`PlayerState.PlayerId` (`Pawn.PlayerState` _asbp_prisonner_dd)))))))

(event `self.OnInteractionInterrupted`
  (params (Actor :type "Actor Object Reference")))

(fn `CanInteract`
  (params (Actor :type "Actor Object Reference"))
  (returns (ReturnValue :type Boolean))
  (return false))

(fn `GetInteractionHoldTime`
  (returns (ReturnValue :type "Float (single-precision)"))
  (return 0.0))

(fn `GetInteractionName`
  (returns (ReturnValue :type String))
  (return "activate the door"))

(fn `GetTypeInteractionName`
  (returns (ReturnValue :type String))
  (return "Press "))

(fn `IsInteractionValid`
  (params (Actor :type "Actor Object Reference"))
  (returns (ReturnValue :type Boolean))
  (return false))

(fn `Open Door with Num Players`
  (params (Door :type "/Game/Blueprints/Environments/Doors/BP_Door Object Reference"))
  (set `/Game/Blueprints/Environments/Doors/BP_Door.PlayerNeeded` 0 Door)
  (`self.Switch Interaction Button` Door true)
  (`self.Event_Multicast_OnButtonPressed` Door))

(fn `Switch Interaction Button`
  (params (Enabled :type Boolean))
  (set `SpawnActor.CanBeUsed` Enabled (cast `/Game/Blueprints/Objects/BP_ButtonInteractable` (`ChildActorComponent.ChildActor` (`self.BP_Button_01`)) :!pure true))
  (set `SpawnActor.CanBeUsed` (`local.Enabled`) (cast `/Game/Blueprints/Objects/BP_ButtonInteractable` (`ChildActorComponent.ChildActor` (`self.BP_Button_02`)) :!pure true)))

(fn `TryInteract`
  (params (Actor :type "Actor Object Reference"))
  (returns (ReturnValue :type Boolean))
  (return false))

(fn `TryStopInteract`
  (params (Actor :type "Actor Object Reference"))
  (returns (ReturnValue :type Boolean))
  (return false))

(fn `UserConstructionScript`
  ;[1 1 1] CHECK IF CLOSE
  (if (not (`self.Close`))
    (`SceneComponent.K2_SetRelativeLocation` (`self.Door_Mesh`) (`self.Distance`) false false)
    (`SceneComponent.K2_SetRelativeLocation` (`self.Door_Mesh`) (`self.Distance`) false false)))