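; BP_SmallDoor is a configurable sliding door with a button, detection box and interaction functions, though the CanInteract and TryInteract logic is unwired.
; Construction sets meshes, centers the box on the button and offsets doors that start open.
; A multicast-named event waits briefly to avoid multiplayer issues, then FlipFlops one of two timelines, chosen by starting state, forward or backward.
; Button material shows red while moving, green when finished.
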(event `self.DetectionArea.OnComponentBeginOverlap`
  (params (OverlappedComponent :type "PrimitiveComponent Object Reference") (OtherActor :type "Actor Object Reference") (OtherComp :type "PrimitiveComponent Object Reference") (OtherBodyIndex :type Integer) (bFromSweep :type Boolean) (SweepResult :type "HitResult Structure (by ref)"))
  ;[0 0 0] BOX DETECT PLAYER
  (set `self.InFrontOf` true))

(event `self.DetectionArea.OnComponentEndOverlap`
  (params (OverlappedComponent :type "PrimitiveComponent Object Reference") (OtherActor :type "Actor Object Reference") (OtherComp :type "PrimitiveComponent Object Reference") (OtherBodyIndex :type Integer))
  ;[0 0 0] BOX DETECT PLAYER
  (set `self.InFrontOf` false))

(event `Event_MulticastMoveDoor`
  (bind _distance (`self.Distance`))
  ;[0 0 0] CAN'T OPEN WHILE DOOR IS MOVING
  (`PrimitiveComponent.SetMaterial` (`self.Button_Mesh`) 0 "/Engine/EngineDebugMaterials/VertexColorViewMode_RedOnly.VertexColorViewMode_RedOnly")
  ;;[0 0 0] DELAY TO AVOID MULTIPLAYER PROBLEMS
  (`KismetSystemLibrary.Delay` 0.5)
  (if (not (`self.IsMoving`))
    (set `self.IsMoving` true)
    ;[0 0 0] CHECK IF CLOSE
    (if (`self.Close`)
      (set `self.isUsable` false)
      (`/Engine/EditorBlueprintResources/StandardMacros.FlipFlop`
        (:`A`
          ;[0 0 0] DOOR MOVEMENT
          (bind (_direction _alpha) (`Timeline|Timeline` :!label _label)
            (:`Update`
              (`SceneComponent.K2_SetRelativeLocation` (`self.Door_Mesh`) (* _alpha _distance) false false))
            (:`Finished`
              (set `self.isUsable` true :!label _label_2)
              (set `self.IsMoving` false)
              (`PrimitiveComponent.SetMaterial` (`self.Button_Mesh`) 0 "/Engine/EngineDebugMaterials/VertexColorViewMode_GreenOnly.VertexColorViewMode_GreenOnly"))))
        (:`B`
          (goto _label :!via `Reverse`)))
      (else
        (`/Engine/EditorBlueprintResources/StandardMacros.FlipFlop`
          (:`A`
            (bind (_direction_2 _alpha_2) (`Timeline|Timeline_0` :!label _label_3)
              (:`Update`
                (`SceneComponent.K2_SetRelativeLocation` (`self.Door_Mesh`) (* _distance _alpha_2) false false))
              (:`Finished`
                (goto _label_2))))
          (:`B`
            (goto _label_3 :!via `Reverse`)))))))

(fn `CanInteract`
  (params (Actor :type "Actor Object Reference"))
  (returns (ReturnValue :type Boolean)))

(fn `GetInteractionHoldTime`
  (returns (ReturnValue :type "Float (single-precision)"))
  (return 0.0))

(fn `GetInteractionName`
  (returns (ReturnValue :type String))
  (return "activate the door "))

(fn `GetTypeInteractionName`
  (returns (ReturnValue :type String))
  (return "Press "))

(fn `IsInteractionValid`
  (params (Actor :type "Actor Object Reference"))
  (returns (ReturnValue :type Boolean))
  (return false))

(fn `TryInteract`
  (params (Actor :type "Actor Object Reference"))
  (returns (ReturnValue :type Boolean)))

(fn `TryStopInteract`
  (params (Actor :type "Actor Object Reference"))
  (returns (ReturnValue :type Boolean))
  (return false))

(fn `UserConstructionScript`
  ;[0 0 0] BOX EXTEND
  (`BoxComponent.SetBoxExtent` (`self.DetectionArea`) (`self.BoxSize`) false)
  ;[0 0 0] CENTER BOX ON  BUTTON
  (`SceneComponent.K2_SetWorldLocation` (`self.DetectionArea`) (`SceneComponent.K2_GetComponentLocation` (`self.Button_Mesh`)) false true)
  ;[0 0 0] SET MESHES
  (`StaticMeshComponent.SetStaticMesh` (`self.Frame_Mesh`) (`self.Frame`))
  (`StaticMeshComponent.SetStaticMesh` (`self.Door_Mesh`) (`self.Door`))
  ;[1 1 1] CHECK IF CLOSE
  (if (not (`self.Close`))
    (`SceneComponent.K2_SetRelativeLocation` (`self.Door_Mesh`) (`self.Distance`) false false)))