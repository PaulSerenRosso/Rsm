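; BP_EditorNote is an editor note actor that displays a designer-entered text note in the level.
; The construction script copies NoteText into the TextNote text component and sizes it by character count, shrinking longer notes linearly within a clamped range.
; It has no runtime logic; its event graph holds only disabled stubs.
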(fn `UserConstructionScript`
  (bind _notetext (`self.NoteText`))
  (`TextRenderComponent.K2_SetText` (`self.TextNote`) _notetext)
  (`TextRenderComponent.SetWorldSize` (`self.TextNote`) (`KismetMathLibrary.FClamp` (- 30.0 (* (`KismetMathLibrary.Conv_IntToDouble` (`KismetStringLibrary.Len` (`KismetTextLibrary.Conv_TextToString` _notetext))) 1.2)) 10.0 30.0)))