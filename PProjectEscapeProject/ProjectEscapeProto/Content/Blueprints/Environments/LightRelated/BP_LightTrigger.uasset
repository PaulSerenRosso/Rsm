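; BP_LightTrigger is an environment light that switches on while something overlaps its trigger zone.
; Begin and end overlap set the PointLight intensity to a fixed value or zero, with no actor filter or overlap count.
; It also implements interaction functions, but these are mostly stubs returning empty or false values.
; Only CanInteract differs, returning InFrontOf for a BP_PrisonnerDD actor.
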(event `self.TriggerZone.OnComponentBeginOverlap`
  (params (OverlappedComponent :type "PrimitiveComponent Object Reference") (OtherActor :type "Actor Object Reference") (OtherComp :type "PrimitiveComponent Object Reference") (OtherBodyIndex :type Integer) (bFromSweep :type Boolean) (SweepResult :type "HitResult Structure (by ref)"))
  (`LightComponent.SetIntensity` (`self.PointLight`) 5000.0))

(event `self.TriggerZone.OnComponentEndOverlap`
  (params (OverlappedComponent :type "PrimitiveComponent Object Reference") (OtherActor :type "Actor Object Reference") (OtherComp :type "PrimitiveComponent Object Reference") (OtherBodyIndex :type Integer))
  (`LightComponent.SetIntensity` (`self.PointLight`) 0.0))

(fn `CanInteract`
  (params (Actor :type "Actor Object Reference"))
  (returns (ReturnValue :type Boolean))
  (cast `/Game/Blueprints/Characters/BP_PrisonnerDD` Actor)
  (return (`self.inFrontOf`)))

(fn `GetInteractionHoldTime`
  (returns (ReturnValue :type "Float (single-precision)"))
  (return 0.0))

(fn `GetInteractionName`
  (returns (ReturnValue :type String))
  (return ""))

(fn `GetTypeInteractionName`
  (returns (ReturnValue :type String))
  (return ""))

(fn `IsInteractionValid`
  (params (Actor :type "Actor Object Reference"))
  (returns (ReturnValue :type Boolean))
  (return false))

(fn `TryInteract`
  (params (Actor :type "Actor Object Reference"))
  (returns (ReturnValue :type Boolean))
  (cast `/Game/Blueprints/Characters/BP_PrisonnerDD` Actor)
  (return false))

(fn `TryStopInteract`
  (params (Actor :type "Actor Object Reference"))
  (returns (ReturnValue :type Boolean))
  (return false))

(fn `UserConstructionScript`)