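; BP_Lightswitch is an interactable wall switch that toggles a set of Lights on and off.
; TriggerZone overlaps set InFrontOf, which CanInteract returns, with no filter on the overlapping actor.
; TryInteract calls a multicast event whose FlipFlop swaps the Button material and each light's visibility, turning lights off first.
; IsInteractionValid and TryInteract always return false, and the name getters return empty strings.
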(event `self.TriggerZone.OnComponentBeginOverlap`
  (params (OverlappedComponent :type "PrimitiveComponent Object Reference") (OtherActor :type "Actor Object Reference") (OtherComp :type "PrimitiveComponent Object Reference") (OtherBodyIndex :type Integer) (bFromSweep :type Boolean) (SweepResult :type "HitResult Structure (by ref)"))
  (set `self.inFrontOf` true))

(event `self.TriggerZone.OnComponentEndOverlap`
  (params (OverlappedComponent :type "PrimitiveComponent Object Reference") (OtherActor :type "Actor Object Reference") (OtherComp :type "PrimitiveComponent Object Reference") (OtherBodyIndex :type Integer))
  (set `self.inFrontOf` false))

(event `Event_MulticastTriggerTrap`
  (`/Engine/EditorBlueprintResources/StandardMacros.FlipFlop`
    (:`A`
      (`PrimitiveComponent.SetMaterial` (`self.Button`) 0 "/Game/Art/Environments/Materials/MaterialInstances/FlatColors/MI_Black.MI_Black")
      (for _array_element (`self.Lights`)
        (`SceneComponent.SetVisibility` (`Light.LightComponent` _array_element) false false)))
    (:`B`
      (`PrimitiveComponent.SetMaterial` (`self.Button`) 0 "/Game/Draft/A.A")
      (for _array_element_2 (`self.Lights`)
        (`SceneComponent.SetVisibility` (`Light.LightComponent` _array_element_2) true false)))))

(fn `CanInteract`
  (params (Actor :type "Actor Object Reference"))
  (returns (ReturnValue :type Boolean))
  (return (`self.inFrontOf`)))

(fn `GetInteractionHoldTime`
  (returns (ReturnValue :type "Float (single-precision)"))
  (return 0.0))

(fn `GetInteractionName`
  (returns (ReturnValue :type String))
  (return ""))

(fn `GetTypeInteractionName`
  (returns (ReturnValue :type String))
  (return ""))

(fn `IsInteractionValid`
  (params (Actor :type "Actor Object Reference"))
  (returns (ReturnValue :type Boolean))
  (return false))

(fn `TryInteract`
  (params (Actor :type "Actor Object Reference"))
  (returns (ReturnValue :type Boolean))
  (`self.Event_MulticastTriggerTrap`)
  (return false))

(fn `TryStopInteract`
  (params (Actor :type "Actor Object Reference"))
  (returns (ReturnValue :type Boolean))
  (return false))

(fn `UserConstructionScript`)