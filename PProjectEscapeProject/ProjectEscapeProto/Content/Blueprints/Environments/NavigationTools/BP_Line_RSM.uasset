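; BP_Line_RSM is a navigation-tool line actor that builds a tinted floor line from meshes along an editable spline.
; Its construction script adds shadowless spline meshes per section, using either whole sections only or an extra one covering the remainder.
; Section length can follow actor X scale, and tangents are clamped to it.
; Optional ground snapping line-traces each spline point, adjusting actor height for the first and repositioning the others.
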(fn `FMovePointToGround`
  (bind (_target_location_x _target_location_y _target_location_z) (`KismetMathLibrary.BreakVector` (`self.Target Location`)))
  (bind (_returnvalue_x _returnvalue_y _returnvalue_z) (`KismetMathLibrary.BreakVector` (`SplineComponent.GetLocationAtSplinePoint` (`self.Spline`) (`self.SplinePointIndex`) "World")))
  (bind (_returnvalue_x_2 _returnvalue_y_2 _returnvalue_z_2) (`KismetMathLibrary.BreakVector` (`SplineComponent.GetLocationAtSplinePoint` (`self.Spline`) (`self.SplinePointIndex`) "World")))
  (bind (_returnvalue_x_3 _returnvalue_y_3) (`KismetMathLibrary.BreakVector` (`self.K2_GetActorLocation` self)))
  (for _index (range (`SplineComponent.GetNumberOfSplinePoints` (`self.Spline`)))
    (set `self.SplinePointIndex` _index)
    (bind (_outhit _returnvalue) (`KismetSystemLibrary.LineTraceSingle` :`Start` (`KismetMathLibrary.MakeVector` _returnvalue_x_2 _returnvalue_y_2 (+ _returnvalue_z_2 (`self.SnapThreshold`))) :`End` (`KismetMathLibrary.MakeVector` _returnvalue_x _returnvalue_y (- _returnvalue_z (`self.SnapThreshold`))) :`TraceChannel` "TraceTypeQuery1" :`DrawTime` 2.0))
    (if _returnvalue
      (set `self.Target Location` (+ (`.Location` (`GameplayStatics.BreakHitResult` _outhit)) (`KismetMathLibrary.MakeVector` 0.0 0.0 (`self.SnapOffset`))))
      (if (== (`self.SplinePointIndex`) 0)
        ;[0 0 0] INDEX 0
        (`self.K2_SetActorLocation` self (`KismetMathLibrary.MakeVector` _returnvalue_x_3 _returnvalue_y_3 _target_location_z) false true)
        (else
          ;[0 0 0] Spline to ground
          (`SplineComponent.SetLocationAtSplinePoint` (`self.Spline`) (`self.SplinePointIndex`) (`self.Target Location`) "World" true)))))
  (return))

(fn `GetEndPosTangent`
  (params (Index :type Integer))
  (returns (Position :type "Vector Structure") (Tangent :type "Vector Structure"))
  (bind _spline (`self.Spline`))
  (bind _returnvalue (* (+ Index 1) (`self.SectionLength`)))
  (return (`SplineComponent.GetLocationAtDistanceAlongSpline` _spline _returnvalue "Local") (`KismetMathLibrary.ClampVectorSize` (`SplineComponent.GetTangentAtDistanceAlongSpline` _spline _returnvalue "Local") 0.0 (`self.SectionLength`))))

(fn `GetStartPosTangent`
  (params (Index :type Integer))
  (returns (Position :type "Vector Structure") (Tangent :type "Vector Structure"))
  (bind _spline (`self.Spline`))
  (bind _returnvalue (* Index (`self.SectionLength`)))
  (return (`SplineComponent.GetLocationAtDistanceAlongSpline` _spline _returnvalue "Local") (`KismetMathLibrary.ClampVectorSize` (`SplineComponent.GetTangentAtDistanceAlongSpline` _spline _returnvalue "Local") 0.0 (`self.SectionLength`))))

(fn `UserConstructionScript`
  (bind _returnvalue_x (`KismetMathLibrary.BreakVector` (`self.GetActorScale3D`)))
  (bind (_meshscale_x _meshscale_y) (`KismetMathLibrary.BreakVector` (`self.MeshScale`)))
  (bind _returnvalue (`KismetMathLibrary.MakeVector2D` _meshscale_x _meshscale_y))
  ;[0 0 0] SNAP MESH
  (set `self.Refresh` false)
  (if (`self.MoveToGround`)
    (`self.FMovePointToGround`))
  (if (`self.SplineScaling`)
    ;[0 0 0] SPLINE SCALING
    (set `self.SectionLength` (* _returnvalue_x 100.0)))
  (if (`self.MeshesFullLength`)
    ;[0 0 0] FULL LENGTH
    (for _index (range (`KismetMathLibrary.FTrunc` (/ (`SplineComponent.GetSplineLength` (`self.Spline`)) (`self.SectionLength`))))
      (set `self.LoopIndex` _index)
      ;[0 0 0] ADD MESH
      (bind _returnvalue_2 (`AddComponent|NODE_AddSplineMeshComponent-0` :!label _label))
      (`KismetArrayLibrary.Array_Add` (`self.MeshArray`) _returnvalue_2)
      (`StaticMeshComponent.SetStaticMesh` _returnvalue_2 (`self.MeshToSpawn`))
      (`SplineMeshComponent.SetStartScale` _returnvalue_2 _returnvalue true)
      (`SplineMeshComponent.SetEndScale` _returnvalue_2 _returnvalue true)
      ;[0 0 0] SETTINGS MESH
      (`PrimitiveComponent.SetCastShadow` _returnvalue_2 false)
      (`PrimitiveComponent.SetAffectDistanceFieldLighting` _returnvalue_2 false)
      ;[0 0 0] SET MATERIALS
      (bind _returnvalue_3 (`KismetMaterialLibrary.CreateDynamicMaterialInstance` "/Game/Art/Environments/Materials/MaterialInstances/RSM/MI_RSM_Floor.MI_RSM_Floor"))
      (`MaterialInstanceDynamic.SetVectorParameterValue` _returnvalue_3 "Tint" (`self.Color`))
      (bind _output_get (set `self.Material` _returnvalue_3))
      (`PrimitiveComponent.SetMaterial` _returnvalue_2 0 _output_get)
      ;[0 0 0] FORWARD AXIS
      (`SplineMeshComponent.SetForwardAxis` _returnvalue_2 "X" true)
      (bind (_position _tangent) (`self.GetStartPosTangent` (`self.LoopIndex`)))
      (bind (_position_2 _tangent_2) (`self.GetEndPosTangent` (`self.LoopIndex`)))
      (`SplineMeshComponent.SetStartAndEnd` _returnvalue_2 _position _tangent _position_2 _tangent_2 true)
      (`PrimitiveComponent.SetCollisionEnabled` _returnvalue_2 (`self.CollisionType`)))
    (else
      ;[0 0 0] SPLINE LENGTH
      (for _index_2 (range (+ (`KismetMathLibrary.FTrunc` (/ (`SplineComponent.GetSplineLength` (`self.Spline`)) (`self.SectionLength`))) 1))
        (set `self.LoopIndex` _index_2)
        (goto _label)))))