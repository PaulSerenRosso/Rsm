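; BP_TriggerSound is a trigger actor that plays a sound at its location when a BP_PrisonnerDD overlaps it.
; A Gate closes after each playback and reopens after the sound's duration plus DelayOffset, preventing retriggers in the meantime.
; The construction script optionally adds a static mesh component with the configured mesh when UseStaticMesh is set.
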(event `self.Trigger.OnComponentBeginOverlap`
  (params (OverlappedComponent :type "PrimitiveComponent Object Reference") (OtherActor :type "Actor Object Reference") (OtherComp :type "PrimitiveComponent Object Reference") (OtherBodyIndex :type Integer) (bFromSweep :type Boolean) (SweepResult :type "HitResult Structure (by ref)"))
  (bind _asbp_prisonner_dd (cast `/Game/Blueprints/Characters/BP_PrisonnerDD` OtherActor))
  (`/Engine/EditorBlueprintResources/StandardMacros.IsValid` _asbp_prisonner_dd
    (:`Is Valid`
      (`/Engine/EditorBlueprintResources/StandardMacros.Gate` false :!label _label
        (:`Exit`
          (`GameplayStatics.PlaySoundAtLocation` (`self.Sound`) (`SceneComponent.K2_GetComponentLocation` (`self.DefaultSceneRoot`)) (struct) 1.0 1.0 0.0 null null null null)
          (`|ExecutionSequence`
            (:`then_0`
              (goto _label :!via `Close`))
            (:`then_1`
              (`KismetSystemLibrary.Delay` (+ (`SoundBase.Duration` (`self.Sound`)) (`self.DelayOffset`)))
              (goto _label :!via `Open`))))))))

(fn `UserConstructionScript`
  (if (`self.UseStaticMesh`)
    (bind _returnvalue (`AddComponent|NODE_AddStaticMeshComponent-0`))
    (`StaticMeshComponent.SetStaticMesh` _returnvalue (`self.StaticMesh`))))