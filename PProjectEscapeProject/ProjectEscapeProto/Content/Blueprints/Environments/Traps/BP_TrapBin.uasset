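; Interactable bin trap that a player arms, which then stuns and afterwards slows the next Pawn to step into it.
; Activation calls a multicast event that enables TriggerTrap overlaps, swaps the Printer material, reveals TrapPreview and plays a sound.
; A Pawn overlap resets visuals, collision and usability for reuse, then applies the stun and, after its duration, the slow.
; A separate interact zone only tracks the InFrontOf flag.
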(event `self.ReceiveBeginPlay`
  (`PrimitiveComponent.SetCollisionResponseToAllChannels` (`self.TriggerTrap`) "ECR_Ignore"))

(event `self.InteractZoneDistributor.OnComponentBeginOverlap`
  (params (OverlappedComponent :type "PrimitiveComponent Object Reference") (OtherActor :type "Actor Object Reference") (OtherComp :type "PrimitiveComponent Object Reference") (OtherBodyIndex :type Integer) (bFromSweep :type Boolean) (SweepResult :type "HitResult Structure (by ref)"))
  ;[1 1 1] DETECTION ZONE TO TRIGGER
  (set `self.inFrontOf` true))

(event `self.InteractZoneDistributor.OnComponentEndOverlap`
  (params (OverlappedComponent :type "PrimitiveComponent Object Reference") (OtherActor :type "Actor Object Reference") (OtherComp :type "PrimitiveComponent Object Reference") (OtherBodyIndex :type Integer))
  ;[1 1 1] DETECTION ZONE TO TRIGGER
  (set `self.inFrontOf` false))

(event `Event_MulticastTrapBin`
  ;[1 1 1] TRAP ACTIVATION
  (`PrimitiveComponent.SetCollisionResponseToAllChannels` (`self.TriggerTrap`) "ECR_Overlap")
  (set `self.CurrentlyActivated` true)
  (if (and (`self.Usable`) (`self.CurrentlyActivated`))
    (`PrimitiveComponent.SetMaterial` (`self.Printer`) 0 "/Engine/VREditor/LaserPointer/LaserPointerMaterialInst.LaserPointerMaterialInst")
    (`SceneComponent.SetHiddenInGame` (`self.TrapPreview`) false false)
    (`GameplayStatics.PlaySound2D` "/Game/Sounds/SoundWave/A_GeneratorHit.A_GeneratorHit" 1.0 1.0 0.0 null null))
  (set `self.Usable` false))

(event `self.TriggerTrap.OnComponentBeginOverlap`
  (params (OverlappedComponent :type "PrimitiveComponent Object Reference") (OtherActor :type "Actor Object Reference") (OtherComp :type "PrimitiveComponent Object Reference") (OtherBodyIndex :type Integer) (bFromSweep :type Boolean) (SweepResult :type "HitResult Structure (by ref)"))
  (bind _array (`|MakeArray` OtherActor))
  ;[1 1 1] BACK TO USABLE STATE
  (`KismetSystemLibrary.DelayUntilNextTick`)
  (if (`self.CurrentlyActivated`)
    (cast `Pawn` OtherActor)
    (`|ExecutionSequence`
      (:`then_0`
        (`PrimitiveComponent.SetMaterial` (`self.Printer`) 0 "/Game/Art/Environments/Materials/MaterialInstances/BlockingMaterials/MI_Obstacles.MI_Obstacles")
        (`KismetSystemLibrary.DelayUntilNextTick`)
        (`SceneComponent.SetHiddenInGame` (`self.TrapPreview`) true false)
        (set `self.CurrentlyActivated` false)
        (set `self.Usable` true)
        (`PrimitiveComponent.SetCollisionResponseToAllChannels` (`self.TriggerTrap`) "ECR_Ignore"))
      (:`then_1`
        (`self.StunCharacters` _array)
        (`KismetSystemLibrary.Delay` (`TweakValueTrapData.StunDuration` (`self.TrapData`)))
        (`self.SlowCharacters` _array)))))

(event `self.ActivateEnvironmentalTrapBP`
  (`self.Event_MulticastTrapBin`))

(fn `GetInteractionName`
  (returns (ReturnValue :type String))
  (return "to trigger the trap"))

(fn `GetTypeInteractionName`
  (returns (ReturnValue :type String))
  (return "Maintain "))

(fn `TryStopInteract`
  (params (Actor :type "Actor Object Reference"))
  (returns (ReturnValue :type Boolean))
  (return false))

(fn `UserConstructionScript`)