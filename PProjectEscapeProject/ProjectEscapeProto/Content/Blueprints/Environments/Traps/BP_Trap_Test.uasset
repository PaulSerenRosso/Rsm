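; BP_Trap_Test is a test trap with a button and light, apparently a placeholder for trap activation feedback.
; Event_MulticastTriggerTrap, if Usable, swaps the button material, lights the RectLight and plays a sound, with a five-second delay before resetting.
; TriggerZone overlaps set InFrontOf, but the interaction functions are stubs that never read it or trigger the trap.
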(event `self.TriggerZone.OnComponentBeginOverlap`
  (params (OverlappedComponent :type "PrimitiveComponent Object Reference") (OtherActor :type "Actor Object Reference") (OtherComp :type "PrimitiveComponent Object Reference") (OtherBodyIndex :type Integer) (bFromSweep :type Boolean) (SweepResult :type "HitResult Structure (by ref)"))
  (set `self.inFrontOf` true))

(event `self.TriggerZone.OnComponentEndOverlap`
  (params (OverlappedComponent :type "PrimitiveComponent Object Reference") (OtherActor :type "Actor Object Reference") (OtherComp :type "PrimitiveComponent Object Reference") (OtherBodyIndex :type Integer))
  (set `self.inFrontOf` false))

(event `Event_MulticastTriggerTrap`
  (if (`self.Usable`)
    (`PrimitiveComponent.SetMaterial` (`self.Button`) 0 "/Engine/VREditor/BasicMeshes/MI_Cube_03.MI_Cube_03")
    (`LightComponent.SetIntensity` (`self.RectLight`) 100000.0)
    (`GameplayStatics.PlaySound2D` "/Game/Sounds/SoundWave/A_AddPoints.A_AddPoints" 1.0 1.0 0.0 null null))
  (set `self.Usable` false)
  (`KismetSystemLibrary.Delay` 5.0)
  (`PrimitiveComponent.SetMaterial` (`self.Button`) 0 "/Engine/EngineDebugMaterials/VertexColorViewMode_GreenOnly.VertexColorViewMode_GreenOnly")
  (`LightComponent.SetIntensity` (`self.RectLight`) 0.0)
  (set `self.Usable` true))

(fn `CanInteract`
  (params (Actor :type "Actor Object Reference"))
  (returns (ReturnValue :type Boolean)))

(fn `GetInteractionHoldTime`
  (returns (ReturnValue :type "Float (single-precision)"))
  (return 0.0))

(fn `GetInteractionName`
  (returns (ReturnValue :type String))
  (return ""))

(fn `GetTypeInteractionName`
  (returns (ReturnValue :type String))
  (return ""))

(fn `IsInteractionValid`
  (params (Actor :type "Actor Object Reference"))
  (returns (ReturnValue :type Boolean))
  (return false))

(fn `TryInteract`
  (params (Actor :type "Actor Object Reference"))
  (returns (ReturnValue :type Boolean)))

(fn `TryStopInteract`
  (params (Actor :type "Actor Object Reference"))
  (returns (ReturnValue :type Boolean))
  (return false))

(fn `UserConstructionScript`)