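; BP_Alarm is an interactable press button, filed under Unused environments, that switches the level into alarm mode.
; TryInteract fires a multicast event, named for moving a door, that runs ButtonPress.
; ButtonPress raises the Escape scalar in MPC_Environments and turns every SpotLight and RectLight actor red, with no way to revert.
; CanInteract always passes, while IsInteractionValid and TryInteract always return false.
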(event `Event_MulticastMoveDoor`
  (`self.ButtonPress`))

(event `ButtonPress`
  (`KismetMaterialLibrary.SetScalarParameterValue` "/Game/Art/Environments/Materials/MPC_Environments.MPC_Environments" "Escape" 1.0)
  (`|ExecutionSequence`
    (:`then_0`
      (bind _outactors (`GameplayStatics.GetAllActorsOfClass` "/Script/Engine.SpotLight"))
      (for _array_element _outactors
        (`LightComponent.SetLightColor` (`SpotLight.SpotLightComponent` _array_element) (struct :`R` 1.0 :`G` 0.020833 :`B` 0.020833 :`A` 1.0) true)))
    (:`then_1`
      (bind _outactors_2 (`GameplayStatics.GetAllActorsOfClass` "/Script/Engine.RectLight"))
      (for _array_element_2 _outactors_2
        (`LightComponent.SetLightColor` (`Light.LightComponent` _array_element_2) (struct :`R` 1.0 :`G` 0.020833 :`B` 0.020833 :`A` 1.0) true)))))

(fn `CanInteract`
  (params (Actor :type "Actor Object Reference"))
  (returns (ReturnValue :type Boolean))
  (return true))

(fn `GetInteractionHoldTime`
  (returns (ReturnValue :type "Float (single-precision)"))
  (return 0.0))

(fn `GetInteractionName`
  (returns (ReturnValue :type String))
  (return "activate alarm mode"))

(fn `GetTypeInteractionName`
  (returns (ReturnValue :type String))
  (return "Press "))

(fn `IsInteractionValid`
  (params (Actor :type "Actor Object Reference"))
  (returns (ReturnValue :type Boolean))
  (return false))

(fn `TryInteract`
  (params (Actor :type "Actor Object Reference"))
  (returns (ReturnValue :type Boolean))
  (`self.Event_MulticastMoveDoor`)
  (return false))

(fn `TryStopInteract`
  (params (Actor :type "Actor Object Reference"))
  (returns (ReturnValue :type Boolean))
  (return false))

(fn `UserConstructionScript`)