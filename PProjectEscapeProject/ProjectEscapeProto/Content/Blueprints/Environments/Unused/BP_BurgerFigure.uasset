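; Burger mascot figure, filed under Unused environments, that greets the player's prisoner character with a Crazy Burger welcome line.
; When a BP_PrisonnerDD overlaps its Box, it has that character print the line and plays an entity roar at the figure's mesh.
; It also draws a debug box on each trigger.
; A SoundPlayed flag and a delay act as a cooldown before the greeting can fire again.
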(event `self.Box.OnComponentBeginOverlap`
  (params (OverlappedComponent :type "PrimitiveComponent Object Reference") (OtherActor :type "Actor Object Reference") (OtherComp :type "PrimitiveComponent Object Reference") (OtherBodyIndex :type Integer) (bFromSweep :type Boolean) (SweepResult :type "HitResult Structure (by ref)"))
  (if (not (`self.SoundPlayed`))
    (bind _asbp_prisonner_dd (cast `/Game/Blueprints/Characters/BP_PrisonnerDD` OtherActor))
    (`/Game/Blueprints/Characters/BP_PrisonnerDD.PrintMascotLine` _asbp_prisonner_dd "Welcome to Crazy Burger, a world of flavour to sink your teeth in !" false)
    (`GameplayStatics.PlaySoundAtLocation` "/Game/Sounds/SoundCue/A_EntitiesRoar.A_EntitiesRoar" (`SceneComponent.K2_GetComponentLocation` (`self.StaticMeshComponent`)) (struct) 1.0 1.0 0.0 null null null null)
    (`KismetSystemLibrary.DrawDebugBox` (0.0 0.0 0.0) (50.0 50.0 50.0))
    (set `self.SoundPlayed` true)
    (`KismetSystemLibrary.Delay` 15.0)
    (set `self.SoundPlayed` false)))

(fn `UserConstructionScript`)