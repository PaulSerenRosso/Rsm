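; BP_LOOT is a lootable prop with a prompt text that yaws toward the player camera each tick.
; Pressing E plays a timeline that fills a radial LoadingCircle material through CompleteRange, then hides the prompt, adds a Niagara effect and clears the Loot flag.
; Leaving the box disables input, but the begin-overlap branch does nothing and EnableInput is unconnected.
; No items are granted, and a debug "Hello" print remains.
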(event `self.ReceiveTick`
  (params (DeltaSeconds :type "Float (single-precision)"))
  (`SceneComponent.K2_SetWorldRotation` (`self.LootText`) (`KismetMathLibrary.MakeRotator` 0.0 0.0 (.yaw (`KismetMathLibrary.FindLookAtRotation` (`self.K2_GetActorLocation`) (`self.K2_GetActorLocation` (`GameplayStatics.GetPlayerCameraManager` 0))))) false false))

(event `self.Box.OnComponentEndOverlap`
  (params (OverlappedComponent :type "PrimitiveComponent Object Reference") (OtherActor :type "Actor Object Reference") (OtherComp :type "PrimitiveComponent Object Reference") (OtherBodyIndex :type Integer))
  (`self.DisableInput` null))

(event `self.Box.OnComponentBeginOverlap`
  (params (OverlappedComponent :type "PrimitiveComponent Object Reference") (OtherActor :type "Actor Object Reference") (OtherComp :type "PrimitiveComponent Object Reference") (OtherBodyIndex :type Integer) (bFromSweep :type Boolean) (SweepResult :type "HitResult Structure (by ref)"))
  (if (`self.Loot`)
    _))

(event `Key|E`
  (params (Key :type "Key Structure"))
  (:`Pressed`
    (if true
      (bind (_direction _alpha) (`Timeline|Timeline`)
        (:`Update`
          (`KismetSystemLibrary.PrintString` "Hello")
          (bind _returnvalue (`KismetMathLibrary.Lerp` 0.0 1.0 _alpha))
          (`MaterialInstanceDynamic.SetScalarParameterValue` (`WidgetComponent.GetMaterialInstance` (`self.LoadingCircle`)) "CompleteRange" _returnvalue)
          (bind _output_get (set `self.Progress` _returnvalue))
          (if (>= _output_get 1.0)
            (`SceneComponent.SetVisibility` (`self.LoadingCircle`) false false)
            (`SceneComponent.SetVisibility` (`self.LootText`) false false)
            (`SceneComponent.SetVisibility` (`self.E`) false false)
            (`AddComponent|NODE_AddNiagaraComponent-0` :`RelativeTransform` (`self.Relative Transform`))
            (set `self.Loot` false)))))))

(fn `UserConstructionScript`)