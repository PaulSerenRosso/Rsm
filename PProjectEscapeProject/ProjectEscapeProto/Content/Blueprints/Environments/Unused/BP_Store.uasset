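; BP_Store is an unused environment store prop with an interactable door, left largely unwired.
; The construction script shows the shop door mesh when Close is set and clears it otherwise.
; Its interaction functions report no valid interaction, though TryInteract uses a FlipFlop to set IsDoorOpen and call an empty open/close multicast.
; Overlap events are empty, and the prompt, input and door-movement logic is disconnected and never runs.
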(event `self.FakeButton.OnComponentBeginOverlap`
  (params (OverlappedComponent :type "PrimitiveComponent Object Reference") (OtherActor :type "Actor Object Reference") (OtherComp :type "PrimitiveComponent Object Reference") (OtherBodyIndex :type Integer) (bFromSweep :type Boolean) (SweepResult :type "HitResult Structure (by ref)")))

(event `self.FakeButton.OnComponentEndOverlap`
  (params (OverlappedComponent :type "PrimitiveComponent Object Reference") (OtherActor :type "Actor Object Reference") (OtherComp :type "PrimitiveComponent Object Reference") (OtherBodyIndex :type Integer)))

(event `Key|E`
  (params (Key :type "Key Structure")))

(event `EventMulticast_OpenCloseStore`)

(fn `CanInteract`
  (params (Actor :type "Actor Object Reference"))
  (returns (ReturnValue :type Boolean))
  (return false))

(fn `GetInteractionHoldTime`
  (returns (ReturnValue :type "Float (single-precision)"))
  (return 0.0))

(fn `GetInteractionName`
  (returns (ReturnValue :type String))
  (return ""))

(fn `GetTypeInteractionName`
  (returns (ReturnValue :type String))
  (return ""))

(fn `IsInteractionValid`
  (params (Actor :type "Actor Object Reference"))
  (returns (ReturnValue :type Boolean))
  (return false))

(fn `TryInteract`
  (params (Actor :type "Actor Object Reference"))
  (returns (ReturnValue :type Boolean))
  (bind _isa (`/Engine/EditorBlueprintResources/StandardMacros.FlipFlop`)
    (:`A`
      (set `self.isDoorOpen?` _isa)
      (`self.EventMulticast_OpenCloseStore`)
      (return true))))

(fn `TryStopInteract`
  (params (Actor :type "Actor Object Reference"))
  (returns (ReturnValue :type Boolean))
  (return false))

(fn `UserConstructionScript`
  (bind _door (`self.Door`))
  (if (`self.Close`)
    (`StaticMeshComponent.SetStaticMesh` _door "/Game/Art/Environments/Meshes/PlaceHolders/SM_Shop_Door_01.SM_Shop_Door_01")
    (else
      (`StaticMeshComponent.SetStaticMesh` _door null))))