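; Online game mode that triggers prisoner pawn color application when a player joins.
; After PostLogin and a short delay, it calls ClientApplyColorFromInstance with true on the new player's BP_PrisonnerDD pawn.
; After a further delay, it loops through PlayerControllers and calls the same function with false on each prisoner pawn.
; The default pawn class override only returns the parent's result.
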(event `self.K2_PostLogin`
  (params (NewPlayer :type "PlayerController Object Reference"))
  (`parent.K2_PostLogin` NewPlayer)
  (`KismetSystemLibrary.Delay` 0.2)
  (bind _asbp_prisonner_dd (cast `/Game/Blueprints/Characters/BP_PrisonnerDD` (`Controller.K2_GetPawn` NewPlayer)))
  (`/Game/Blueprints/Characters/BP_PrisonnerDD.Client_ApplyColorFromInstance` _asbp_prisonner_dd true)
  (`KismetSystemLibrary.Delay` 1.0)
  (for _array_element (`self.PlayerControllers`)
    (bind _asbp_prisonner_dd_2 (cast `/Game/Blueprints/Characters/BP_PrisonnerDD` (`Controller.K2_GetPawn` _array_element)))
    (`/Game/Blueprints/Characters/BP_PrisonnerDD.Client_ApplyColorFromInstance` _asbp_prisonner_dd_2 false)))

(fn `GetDefaultPawnClassForController`
  (params (InController :type "Controller Object Reference"))
  (returns (ReturnValue :type "Object Class Reference"))
  (bind _returnvalue (`parent.GetDefaultPawnClassForController` InController))
  (return _returnvalue))

(fn `UserConstructionScript`)