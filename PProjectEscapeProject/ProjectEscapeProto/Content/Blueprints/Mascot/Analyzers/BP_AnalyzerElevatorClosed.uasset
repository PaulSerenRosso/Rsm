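; Mascot analyzer that detects when the player fails to board the elevator before it closes.
; Its MascotTagAnalyseMetrics function reads the mascot's ElevatorClosed knowledge as a template bool.
; If that is true and the controlled Prisoner's online player state has not succeeded to escape, it returns the IsPrisonerFailToEnterOnElevator tag.
; Otherwise it returns no tag.
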(fn `MascotTagAnalyseMetrics`
  (returns (ReturnValue :type "EMascotTag Enum"))
  (cast `MyTemplateBool` (`Mascot.GetSpecificKnowledge` (`self.MyMascot`) "ElevatorClosed")
    (:`then`
      (if (not (`OnlinePlayerState.SucceedToEscape` (cast `OnlinePlayerState` (`Pawn.PlayerState` (cast `Prisoner` (`Controller.K2_GetPawn` (`Mascot.PC` (`self.MyMascot`))) :!pure true)) :!pure true)))
        (return "IsPrisonerFailToEnterOnElevator")
        (else
          _)))
    (:`CastFailed`
      _))
  (return "None"))