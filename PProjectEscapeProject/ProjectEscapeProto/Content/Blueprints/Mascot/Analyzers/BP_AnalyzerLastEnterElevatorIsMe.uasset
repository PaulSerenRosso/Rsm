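; BP_AnalyzerLastEnterElevatorIsMe is a mascot analyzer that detects whether the prisoner recorded as entering the elevator is the mascot's own player.
; It reads the PrisonerEnteredInElevator knowledge from the mascot as an integer and compares it to the prisoner controller's personal player ID.
; A match returns the IsPrisonerEnteredInElevator tag, while a mismatch or failed cast returns None.
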(fn `MascotTagAnalyseMetrics`
  (returns (ReturnValue :type "EMascotTag Enum"))
  (bind _asmy_template_int (cast `MyTemplateInt` (`Mascot.GetSpecificKnowledge` (`self.MyMascot`) "PrisonerEnteredInElevator"))
    (:`then`
      (bind _asbp_prisoner_controller (cast `/Game/Blueprints/Characters/BP_PrisonerController` (`Mascot.PC` (`self.MyMascot`)))
        (:`then`
          (if (== (`PrisonerController.GetPersonalPlayerID` _asbp_prisoner_controller) (`MyTemplateInt.IntValue` _asmy_template_int))
            (return "IsPrisonerEnteredInElevator")
            (else
              _)))
        (:`CastFailed`
          _)))
    (:`CastFailed`
      _))
  (return "None"))