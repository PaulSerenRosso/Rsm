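; Eye-shaped surveillance camera that turns to watch the player and blinks its eyelids via a timeline started after a random delay.
; A BP_PrisonnerDD entering the box starts a looping timer that yaws the arm and pitches the head, within a clamp, toward player pawn 0.
; Exiting resets rotations from the cached base rotation but never clears the timer, so tracking resumes.
; StartRandomBlinkLoop is an empty stub.
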(event `StartRandomBlinkLoop`)

(event `self.ReceiveBeginPlay`
  (set `self.BaseRot` (`SceneComponent.K2_GetComponentRotation` (`self.SM_Arm01`)))
  (`self.StartRandomBlinkLoop`)
  (`KismetSystemLibrary.Delay` (`KismetMathLibrary.RandomFloatInRange` 1.0 5.0))
  (bind (_direction _blinkalpha) (`Timeline|BlinkTimeline`)
    (:`Update`
      (`SceneComponent.K2_SetRelativeRotation` (`self.SM_UP_Eyelid`) (`KismetMathLibrary.RLerp` (struct) (struct :`Pitch` -70.0) _blinkalpha) false false)
      (`SceneComponent.K2_SetRelativeRotation` (`self.SM_Down_Eyelid`) (`KismetMathLibrary.RLerp` (struct) (struct :`Pitch` 30.0) _blinkalpha) false false))))

(event `self.Box.OnComponentBeginOverlap`
  (params (OverlappedComponent :type "PrimitiveComponent Object Reference") (OtherActor :type "Actor Object Reference") (OtherComp :type "PrimitiveComponent Object Reference") (OtherBodyIndex :type Integer) (bFromSweep :type Boolean) (SweepResult :type "HitResult Structure (by ref)"))
  (cast `/Game/Blueprints/Characters/BP_PrisonnerDD` OtherActor)
  (`KismetSystemLibrary.K2_SetTimer` null "FollowPlayer" 0.05 true))

(event `FollowPlayer`
  (bind (_baserot_roll _baserot_pitch) (`KismetMathLibrary.BreakRotator` (`self.BaseRot`)))
  (bind _returnvalue (`self.K2_GetActorLocation` (`GameplayStatics.GetPlayerPawn` 0)))
  (bind (_returnvalue_roll _returnvalue_pitch) (`KismetMathLibrary.BreakRotator` (`KismetMathLibrary.FindLookAtRotation` (`SceneComponent.K2_GetComponentLocation` (`self.SM_UP_EyedviseCam`)) _returnvalue)))
  (bind (_returnvalue_roll_2 _returnvalue_pitch_2 _returnvalue_yaw) (`KismetMathLibrary.BreakRotator` (`KismetMathLibrary.FindLookAtRotation` (`SceneComponent.K2_GetComponentLocation` (`self.SM_Arm01`)) _returnvalue)))
  (`SceneComponent.K2_SetWorldRotation` (`self.SM_Arm01`) (`KismetMathLibrary.MakeRotator` _baserot_roll _baserot_pitch _returnvalue_yaw) false false)
  (`SceneComponent.K2_SetRelativeRotation` (`self.SM_UP_EyedviseCam`) (`KismetMathLibrary.MakeRotator` 0.0 (`KismetMathLibrary.ClampAngle` _returnvalue_pitch -50.0)) false false))

(event `self.Box.OnComponentEndOverlap`
  (params (OverlappedComponent :type "PrimitiveComponent Object Reference") (OtherActor :type "Actor Object Reference") (OtherComp :type "PrimitiveComponent Object Reference") (OtherBodyIndex :type Integer))
  (bind (_baserot_roll _baserot_pitch _baserot_yaw) (`KismetMathLibrary.BreakRotator` (`self.BaseRot`)))
  (bind (_baserot_roll_2 _baserot_pitch_2 _baserot_yaw_2) (`KismetMathLibrary.BreakRotator` (`self.BaseRot`)))
  (cast `/Game/Blueprints/Characters/BP_PrisonnerDD` OtherActor)
  (`SceneComponent.K2_SetWorldRotation` (`self.SM_Arm01`) (`KismetMathLibrary.MakeRotator` _baserot_roll _baserot_pitch _baserot_yaw) false false)
  (`SceneComponent.K2_SetRelativeRotation` (`self.SM_UP_EyedviseCam`) (`KismetMathLibrary.MakeRotator` _baserot_roll_2 _baserot_pitch_2 _baserot_yaw_2) false false))

(fn `UserConstructionScript`)