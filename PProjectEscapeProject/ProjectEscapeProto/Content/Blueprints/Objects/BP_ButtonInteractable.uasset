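; BP_ButtonInteractable is a button interactable that can only be used once all of its associated rooms have been opened.
; Its construction script attaches the interaction root to the item mesh, with the interaction sphere and widget under that root.
; The CanInteract override checks every RoomsAssimilited entry against RoomsOpened in OnlineGameState, then defers to the parent check.
; A missing room or failed game state cast blocks interaction.
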(fn `CanInteract`
  (params (Actor :type "Actor Object Reference"))
  (returns (ReturnValue :type Boolean))
  (bind _asonline_game_state (cast `OnlineGameState` (`GameplayStatics.GetGameState`))
    (:`then`
      (for _array_element (`self.RoomsAssimilited`)
        (if (not (`KismetArrayLibrary.Array_Contains` (`OnlineGameState.RoomsOpened` _asonline_game_state) _array_element))
          (return false)))
      (bind _returnvalue (`parent.CanInteract` Actor))
      (return _returnvalue))
    (:`CastFailed`
      (return false))))

(fn `UserConstructionScript`
  (bind _interactionroot (`self.InteractionRoot`))
  (`SceneComponent.K2_AttachToComponent` _interactionroot (`self.ItemMesh`) "None" "KeepRelative" "KeepRelative" "KeepRelative" true)
  (`SceneComponent.K2_AttachToComponent` (`self.InteractionSphere`) _interactionroot "None" "KeepRelative" "KeepRelative" "KeepRelative" true)
  (`SceneComponent.K2_AttachToComponent` (`self.InteractionWidget`) _interactionroot "None" "KeepRelative" "KeepRelative" "KeepRelative" true))