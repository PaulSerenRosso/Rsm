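; Interactable HUB button that briefly opens the tutorial doors tagged "First".
; CanInteract requires every room in RoomsAssimilited to be open in OnlineGameState, plus the parent check.
; TryInteract turns the button's dynamic material red, then on authority opens the doors and prints a mascot line on player 0's prisoner.
; After delays, authority closes the doors and restores the white emissive.
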(event `self.ReceiveBeginPlay`
  (bind _cube (`self.Cube`))
  (bind _returnvalue (`PrimitiveComponent.CreateDynamicMaterialInstance` _cube 0 "/Game/Art/Environments/Materials/MaterialInstances/Props/MI_Buton.MI_Buton" "None"))
  (`PrimitiveComponent.SetMaterial` _cube 0 _returnvalue)
  (set `self.Material Button` _returnvalue)
  (`MaterialInstanceDynamic.SetVectorParameterValue` (`self.Material Button`) "EmissiveColor" (struct :`R` 1.0 :`G` 1.0 :`B` 1.0 :`A` 1.0)))

(event `TriggerButton`
  (`MaterialInstanceDynamic.SetVectorParameterValue` (`self.Material Button`) "EmissiveColor" (struct :`R` 1.0 :`A` 1.0))
  (`/Engine/EditorBlueprintResources/ActorMacros.Switch Has Authority`
    (:`Authority`
      (bind _outactors (`GameplayStatics.GetAllActorsOfClassWithTag` "/Game/Blueprints/Design/BP_Door_Tutorial.BP_Door_Tutorial_C" "First"))
      (for _array_element _outactors
        (`/Game/Blueprints/Design/BP_Door_Tutorial.Open Doors` _array_element)
        (bind _asbp_prisonner_dd (cast `/Game/Blueprints/Characters/BP_PrisonnerDD` (`GameplayStatics.GetPlayerCharacter` 0)))
        (`/Game/Blueprints/Characters/BP_PrisonnerDD.PrintMascotLine` _asbp_prisonner_dd "Nice work ! Now wait for the other prisonners to start a program" false)
        (`KismetSystemLibrary.Delay` 3.0)
        (bind _outactors_2 (`GameplayStatics.GetAllActorsOfClassWithTag` "/Game/Blueprints/Design/BP_Door_Tutorial.BP_Door_Tutorial_C" "First"))
        (for _array_element_2 _outactors_2
          (`/Game/Blueprints/Design/BP_Door_Tutorial.Close Doors` _array_element_2)
          (`KismetSystemLibrary.Delay` 2.0)
          (`MaterialInstanceDynamic.SetVectorParameterValue` (`self.Material Button`) "EmissiveColor" (struct :`R` 1.0 :`G` 1.0 :`B` 1.0 :`A` 1.0)))))))

(fn `CanInteract`
  (params (Actor :type "Actor Object Reference"))
  (returns (ReturnValue :type Boolean))
  (bind _asonline_game_state (cast `OnlineGameState` (`GameplayStatics.GetGameState`))
    (:`then`
      (for _array_element (`self.RoomsAssimilited`)
        (if (not (`KismetArrayLibrary.Array_Contains` (`OnlineGameState.RoomsOpened` _asonline_game_state) _array_element))
          (return false)))
      (bind _returnvalue (`parent.CanInteract` Actor))
      (return _returnvalue))
    (:`CastFailed`
      (return false))))

(fn `TryInteract`
  (params (Actor :type "Actor Object Reference"))
  (returns (ReturnValue :type Boolean))
  (`self.TriggerButton`)
  (return false))

(fn `UserConstructionScript`
  (`SceneComponent.K2_AttachToComponent` (`self.InteractionRoot`) (`self.ItemMesh`) "None" "KeepRelative" "KeepRelative" "KeepRelative" true)
  (`SceneComponent.K2_AttachToComponent` (`self.InteractionSphere`) (`self.InteractionRoot`) "None" "KeepRelative" "KeepRelative" "KeepRelative" true))