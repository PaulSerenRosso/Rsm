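; Hold-to-interact launch button that readies players up for game start and displays a ready-count widget on its mesh.
; The WBP_Ready render target feeds a dynamic material, reapplied by a looping timer.
; Interacting updates that widget with a fixed zero index and changes the prompt to un-ready.
; StartCountdown runs once and, if player character 0 is locally controlled, opens the doors, adds the start-program widget and plays start music.
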(event `UpdateWidget`
  (params (Index :type Integer))
  (bind _aswbp_ready (cast `/Game/Blueprints/Widgets/WBP_Ready` (`WidgetComponent.GetWidget` (`self.Widget`))))
  (`/Game/Blueprints/Widgets/WBP_Ready.UpdatePlayerNb` _aswbp_ready Index))

(event `self.StartCountdown`
  (params (_CountDownTimer :type "Float (single-precision)"))
  (`/Engine/EditorBlueprintResources/StandardMacros.DoOnce` false
    (:`Completed`
      (if (`Pawn.IsLocallyControlled` (`GameplayStatics.GetPlayerCharacter` 0))
        (`/Game/Blueprints/Design/BP_Door_Tutorial.Open Doors` (`self.BP_Door`))
        (bind _returnvalue (`|CreateWidget` "/Game/Blueprints/Widgets/WBP_StartProgram.WBP_StartProgram_C" (`GameplayStatics.GetPlayerController` 0)))
        (`UserWidget.AddToViewport` _returnvalue 0)
        (`GameplayStatics.PlaySound2D` "/Game/Sounds/SoundCue/Music/A_Music_Start.A_Music_Start" 1.0 1.0 0.0 null null)))))

(event `self.ReceiveBeginPlay`
  (`KismetSystemLibrary.K2_SetTimer` null "SetRenderTarget" 0.1 true))

(fn `GetInteractionName`
  (returns (ReturnValue :type String))
  (bind _returnvalue (`parent.GetInteractionName`))
  (return _returnvalue))

(fn `GetTypeInteractionName`
  (returns (ReturnValue :type String))
  (return "Hold "))

(fn `SetRenderTarget`
  (`/Engine/EditorBlueprintResources/StandardMacros.IsValid` (`self.MID`)
    (:`Is Valid`
      (`MaterialInstanceDynamic.SetTextureParameterValue` (`self.MID`) "Texture" (`WidgetComponent.GetRenderTarget` (`self.Widget`))))))

(fn `TryInteract`
  (params (Actor :type "Actor Object Reference"))
  (returns (ReturnValue :type Boolean))
  (bind _returnvalue (`parent.TryInteract` Actor))
  (`self.UpdateWidget` 0)
  (set `self.InteractableName` "To not be ready")
  (return _returnvalue))

(fn `UserConstructionScript`
  (bind _returnvalue (`KismetMaterialLibrary.CreateDynamicMaterialInstance` (`self.Material`)))
  (set `self.MID` _returnvalue)
  (`PrimitiveComponent.SetMaterial` (`self.ItemMesh`) 1 (`self.MID`))
  (`MaterialInstanceDynamic.SetTextureParameterValue` (`self.MID`) "Texture" (`WidgetComponent.GetRenderTarget` (`self.Widget`))))