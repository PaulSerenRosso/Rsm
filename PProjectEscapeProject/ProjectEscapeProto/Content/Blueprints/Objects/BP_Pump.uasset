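; Interactable balloon pump ("Stay" to "arise balloon") with progress text, balloon scaling and an explosion on failure.
; Authority Tick resets HealthRatio to zero and scales the mesh from it, so the balloon stays at zero size.
; The failure handler plays red material, swelling, sound, Niagara and fire, printing if fire collision is overlapped.
; Binding that handler, the success trigger and actor destruction sit in unconnected nodes.
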(event `EventBalloon`
  (bind _minscale (`self.MinScale`))
  ;[0 0 0] BALLOON EVENT
  (bind _output_get (set `self.HealthRatio` 0.0))
  (bind _output_get_2 (set `self.Balloon Scale` (* (+ _minscale (- (`self.MaxScale`) _minscale)) (`KismetMathLibrary.Conv_DoubleToVector` _output_get))))
  (`SceneComponent.SetRelativeScale3D` (`self.ItemMesh`) _output_get_2))

(event `self.ReceiveTick`
  (params (DeltaSeconds :type "Float (single-precision)"))
  (`/Engine/EditorBlueprintResources/ActorMacros.Switch Has Authority`
    (:`Authority`
      (`self.EventBalloon`))
    (:`Remote`
      _))
  (`TextRenderComponent.K2_SetText` (`self.ProgressText`) (`KismetTextLibrary.Conv_DoubleToText` (`self.HealthRatio`) "HalfToEven")))

(event `self.ReceiveBeginPlay`
  ;[0 0 0] BIND EVENT
  (`SceneComponent.SetRelativeScale3D` (`self.ItemMesh`) (0.0 0.0 0.0)))

(event `OnBalloonFinished_Event` :!signature `self.OnBalloonFinished`
  (params (WithSuccess :type Boolean))
  (bind _balloonlocation (`self.BalloonLocation`))
  ;[0 0 0] BIND EVENT
  (`self.Multicast_OnBalloonFinished`)
  (if (not WithSuccess)
    (`/Engine/EditorBlueprintResources/StandardMacros.DoOnce` false
      (:`Completed`
        ;[0 0 0] EXPLOSION !!!
        (`PrimitiveComponent.SetMaterial` (`self.ItemMesh`) 0 "/Engine/EngineDebugMaterials/VertexColorViewMode_RedOnly.VertexColorViewMode_RedOnly")
        (`KismetSystemLibrary.Delay` 0.8)
        (`SceneComponent.SetRelativeScale3D` (`self.ItemMesh`) (+ (`self.Balloon Scale`) (0.25 0.25 0.25)))
        (`KismetSystemLibrary.Delay` 0.5)
        (`GameplayStatics.PlaySoundAtLocation` "/Game/Sounds/SoundCue/A_BalloonExplosed.A_BalloonExplosed" _balloonlocation (struct) 1.0 1.0 0.0 null null null null)
        (`AddComponent|NODE_AddNiagaraComponent-1` :`RelativeTransform` (`KismetMathLibrary.Conv_VectorToTransform` _balloonlocation))
        (`KismetSystemLibrary.Delay` 1.0)
        (`SceneComponent.SetVisibility` (`self.Fire`) true false)
        (if (`self.OnFire`)
          (`KismetSystemLibrary.PrintString` "On fire !"))))))

(event `Multicast_OnBalloonFinished`
  ;[0 0 0] END EVENT
  (`SceneComponent.SetHiddenInGame` (`self.ItemMesh`) true false))

(event `Multicast_SucceedBalloon`
  ;[0 0 0] END EVENT
  (`PrimitiveComponent.SetMaterial` (`self.ItemMesh`) 0 "/Engine/EngineDebugMaterials/VertexColorViewMode_GreenOnly.VertexColorViewMode_GreenOnly"))

(event `self.FireCollision.OnComponentBeginOverlap`
  (params (OverlappedComponent :type "PrimitiveComponent Object Reference") (OtherActor :type "Actor Object Reference") (OtherComp :type "PrimitiveComponent Object Reference") (OtherBodyIndex :type Integer) (bFromSweep :type Boolean) (SweepResult :type "HitResult Structure (by ref)"))
  (set `self.OnFire` true))

(event `self.FireCollision.OnComponentEndOverlap`
  (params (OverlappedComponent :type "PrimitiveComponent Object Reference") (OtherActor :type "Actor Object Reference") (OtherComp :type "PrimitiveComponent Object Reference") (OtherBodyIndex :type Integer))
  (set `self.OnFire` false))

(fn `GetInteractionName`
  (returns (ReturnValue :type String))
  (return "arise balloon"))

(fn `GetTypeInteractionName`
  (returns (ReturnValue :type String))
  (return "Stay "))

(fn `UserConstructionScript`)