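; BP_SpawnTrapManager spawns incapacitating traps at randomized locations when an online match starts.
; On the authority only, it binds to the start-game event of BP_OnlineGameMode.
; When that fires, it shuffles the "Traps" tagged actors cached in InfoManager and spawns BP_IncapacitedTrap at the transforms of the first NbNecessary entries.
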(event `self.ReceiveBeginPlay`
  (`/Engine/EditorBlueprintResources/ActorMacros.Switch Has Authority`
    (:`Authority`
      (bind _asbp_online_game_mode (cast `/Game/Blueprints/GM/BP_OnlineGameMode` (`GameplayStatics.GetGameMode`)))
      (add `OnlineGameMode.OnStartGame` _asbp_online_game_mode (delegate `OnStartGame_Event`)))))

(event `OnStartGame_Event`
  (`self.SpawnTraps`))

(event `SpawnTraps`
  (bind _actors (break `ArrayOfActors` (`BlueprintMapLibrary.Map_Find` (`MapInfoManager.AllTaggedActorsBis` (`self.InfoManager`)) "Traps")))
  (`KismetArrayLibrary.Array_Shuffle` _actors)
  (set `self.Actors` _actors)
  (for _index (range (`self.NbNecessary`))
    (`|SpawnActorFromClass` "/Game/Blueprints/Objects/Items/BP_IncapacitedTrap.BP_IncapacitedTrap_C" (`self.GetTransform` (`|GetArrayItem` (`self.Actors`) _index)) "Undefined" "MultiplyWithRoot" null null)))

(fn `UserConstructionScript`)