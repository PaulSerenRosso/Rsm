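; Placeable trap item that catches prisoners, with valid/invalid placement previews and mesh swaps for armed and triggered states.
; Activation briefly shows a trapped widget to the locally controlled prisoner, makes a loud noise at the trap, then plays a dog growl and destroys itself.
; On box overlap, the server waits briefly and, if activation has flagged it, snaps the prisoner onto the trap and multicasts the new position.
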(event `self.ReceiveBeginPlay`
  (add `Trap.OnActivateTrap` (delegate `OnActivateTrap_Event`)))

(event `OnActivateTrap_Event`
  (`GameplayStatics.PlaySoundAtLocation` "/Game/Sounds/SoundCue/A_TrapActivation_Cue.A_TrapActivation_Cue" (`SceneComponent.K2_GetComponentLocation` (`self.ItemMesh`)) (struct) 1.0 1.0 0.0 null null null null))

(event `self.InvalidPrevisuMaterialBP`
  (bind _itemmesh (`self.ItemMesh`))
  (`StaticMeshComponent.SetStaticMesh` (`self.ItemMesh`) "/Game/Art/Environments/Meshes/Items/SM_Trap.SM_Trap")
  (for _index (range (`KismetArrayLibrary.Array_Length` (`MeshComponent.GetMaterials` _itemmesh)))
    (`PrimitiveComponent.SetMaterial` _itemmesh _index "/Game/Art/Environments/Materials/MaterialInstances/MI_Previz_Trap_Invalid.MI_Previz_Trap_Invalid")))

(event `self.ValidPrevisuMaterialBP`
  (bind _itemmesh (`self.ItemMesh`))
  (`StaticMeshComponent.SetStaticMesh` (`self.ItemMesh`) "/Game/Art/Environments/Meshes/Items/SM_Trap.SM_Trap")
  (for _index (range (`KismetArrayLibrary.Array_Length` (`MeshComponent.GetMaterials` _itemmesh)))
    (`PrimitiveComponent.SetMaterial` _itemmesh _index "/Game/Art/Environments/Materials/MaterialInstances/MI_Previz_Trap_Valid.MI_Previz_Trap_Valid")))

(event `self.BP_ArmTrap`
  (`StaticMeshComponent.SetStaticMesh` (`self.ItemMesh`) "/Game/Art/Environments/Meshes/Items/SM_TrapArm.SM_TrapArm"))

(event `self.BP_ActivateTrap`
  (params (StunnedActor :type "Actor Object Reference"))
  (set `self.CanBeUsed` false)
  (set `self.ActivateTrapTrue` true)
  (`|ExecutionSequence`
    (:`then_0`
      (bind _asprisoner (cast `Prisoner` StunnedActor))
      (if (`Pawn.IsLocallyControlled` _asprisoner)
        (bind _returnvalue (`|CreateWidget` "/Game/Blueprints/Widgets/WBP_Trapped.WBP_Trapped_C"))
        (`UserWidget.AddToViewport` _returnvalue 0)
        (`KismetSystemLibrary.Delay` 2.5)
        (`Widget.RemoveFromParent` _returnvalue)))
    (:`then_1`
      (`StaticMeshComponent.SetStaticMesh` (`self.ItemMesh`) "/Game/Art/Environments/Meshes/Items/SM_TrapActivate.SM_TrapActivate")
      (`FunctionsUtilities.Server_MakeNoise` StunnedActor StunnedActor (`self.K2_GetActorLocation`) 600.0 30000)
      (`KismetSystemLibrary.Delay` 2.0)
      (`GameplayStatics.PlaySoundAtLocation` "/Game/Sounds/SoundWave/A_DogGrowling.A_DogGrowling" (`SceneComponent.K2_GetComponentLocation` (`self.ItemMesh`)) (struct) 1.0 1.0 0.0 null null null null)
      (`self.K2_DestroyActor`))))

(event `self.BoxComponent.OnComponentBeginOverlap`
  (params (OverlappedComponent :type "PrimitiveComponent Object Reference") (OtherActor :type "Actor Object Reference") (OtherComp :type "PrimitiveComponent Object Reference") (OtherBodyIndex :type Integer) (bFromSweep :type Boolean) (SweepResult :type "HitResult Structure (by ref)"))
  (bind (_returnvalue_x _returnvalue_y _returnvalue_z) (`KismetMathLibrary.BreakVector` (`self.K2_GetActorLocation`)))
  (`/Engine/EditorBlueprintResources/ActorMacros.Switch Has Authority`
    (:`Authority`
      (`KismetSystemLibrary.Delay` 0.05)
      (if (`self.ActivateTrapTrue`)
        (bind _asbp_prisonner_dd (cast `/Game/Blueprints/Characters/BP_PrisonnerDD` OtherActor))
        (bind _returnvalue (`KismetMathLibrary.MakeVector` _returnvalue_x _returnvalue_y (+ _returnvalue_z (`CapsuleComponent.GetScaledCapsuleHalfHeight` (`Character.CapsuleComponent` _asbp_prisonner_dd)))))
        (`self.K2_SetActorLocation` _asbp_prisonner_dd _returnvalue false false)
        (`self.Multicast_SwitchPosition` _asbp_prisonner_dd _returnvalue)
        (set `self.ActivateTrapTrue` false)))))

(event `Multicast_SwitchPosition`
  (params (Target :type "Actor Object Reference") (NewLocation :type "Vector Structure"))
  (`self.K2_SetActorLocation` Target NewLocation false false))

(fn `UserConstructionScript`)