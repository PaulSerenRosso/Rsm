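; BP_SlowingTrap is a trap item that, despite its name, contains no slowing logic in these graphs.
; When a BP_PrisonnerDD overlaps its sphere, it makes the Cylinder component visible, and nothing here hides it again.
; Two placement-preview events loop over the item mesh's material slots: the valid one applies BasicAsset03, while the invalid one sets no material.
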(event `self.Sphere_0.OnComponentBeginOverlap`
  (params (OverlappedComponent :type "PrimitiveComponent Object Reference") (OtherActor :type "Actor Object Reference") (OtherComp :type "PrimitiveComponent Object Reference") (OtherBodyIndex :type Integer) (bFromSweep :type Boolean) (SweepResult :type "HitResult Structure (by ref)"))
  (cast `/Game/Blueprints/Characters/BP_PrisonnerDD` OtherActor)
  (`SceneComponent.SetVisibility` (`self.Cylinder`) true false))

(event `self.InvalidPrevisuMaterialBP`
  (bind _itemmesh (`self.ItemMesh`))
  (for _index (range (`KismetArrayLibrary.Array_Length` (`MeshComponent.GetMaterials` _itemmesh)))
    (`PrimitiveComponent.SetMaterial` _itemmesh _index null)))

(event `self.ValidPrevisuMaterialBP`
  (bind _itemmesh (`self.ItemMesh`))
  (for _index (range (`KismetArrayLibrary.Array_Length` (`MeshComponent.GetMaterials` _itemmesh)))
    (`PrimitiveComponent.SetMaterial` _itemmesh _index "/Engine/MapTemplates/Materials/BasicAsset03.BasicAsset03")))

(fn `UserConstructionScript`)