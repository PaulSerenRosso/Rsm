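; BP_PrisonID is a prison ID actor that fills its text components once at BeginPlay.
; It shows a fixed placeholder name, a random code and the current time and date through FormatText.
; The day and month padding selects between literal template strings, so the actual day and month numbers never reach the date text.
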(event `self.ReceiveBeginPlay`
  (bind _returnvalue (`KismetMathLibrary.Now`))
  (bind _returnvalue_2 (`KismetMathLibrary.Now`))
  (bind _output_get (set `self.ID` "PSEUDO"))
  (bind _output_get_2 (set `self.Code` (`KismetMathLibrary.RandomIntegerInRange` 0 100)))
  (`TextRenderComponent.K2_SetText` (`self.Hour`) (`|FormatText` "{Hour}:{Minuter}" (`KismetMathLibrary.GetHour` _returnvalue_2) (`KismetMathLibrary.GetMinute` _returnvalue_2)))
  (`TextRenderComponent.K2_SetText` (`self.IDtext`) (`|FormatText` " {ID}" _output_get))
  (`TextRenderComponent.K2_SetText` (`self.Datetexte`) (`|FormatText` "{Day}/{Month}/{Year}" (`KismetMathLibrary.GetYear` _returnvalue) (`KismetMathLibrary.SelectString` "\"0\" +{Day}" "{Day}" (< (`KismetMathLibrary.GetDay` _returnvalue) 10)) (`KismetMathLibrary.SelectString` "\"0\"+{Month}" "{Month}" (< (`KismetMathLibrary.GetMonth` _returnvalue) 10))))
  (`TextRenderComponent.K2_SetText` (`self.Codetext`) (`|FormatText` " {Code}" _output_get_2)))

(fn `UserConstructionScript`)