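; Player action component that shows the interaction prompt on the HUD when hovering over interactables.
; On multicast init it binds to the hover-interactable event, only for the locally controlled prisoner.
; Each hover update looks up the first key mapped to IA_Interact through Enhanced Input, so the prompt shows the current binding.
; It passes that key name, the hit state, interaction name and input mode to the first-person character's HUD widget.
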(event `self.EventMulticastInitAction`
  (params (InPrisoner :type "Object Object Reference"))
  (if (`Pawn.IsLocallyControlled` InPrisoner)
    (add `self.OnHoverInteractable` (delegate `OnHoverInteraction`))))

(event `OnHoverInteraction` :!signature `self.OnHoverInteractable`
  (params (IsHit :type Boolean) (InteractionName :type String) (ModeOfInputUtilisation :type String))
  (bind _as_bp_first_person_character (`self.As BP First Person Character`))
  (bind _ingamewidget (`/Game/Blueprints/Characters/BP_PrisonnerDD.InGameWidget` _as_bp_first_person_character))
  (bind _returnvalue (`EnhancedInputSubsystemInterface.QueryKeysMappedToAction` (pcsubsystem `EnhancedInputLocalPlayerSubsystem` (`GameplayStatics.GetPlayerController` 0)) "/Game/Blueprints/Inputs/Actions/IA_Interact.IA_Interact"))
  (`/Engine/EditorBlueprintResources/StandardMacros.IsValid` _as_bp_first_person_character
    (:`Is Valid`
      (if (`KismetSystemLibrary.IsValid` _ingamewidget)
        (if (> (`KismetArrayLibrary.Array_Length` _returnvalue) 0)
          (`/Game/Blueprints/Widgets/WBP_HUD.EnableAndRefreshPickItemText` (`/Game/Blueprints/Widgets/WBP_InGameWidget.WBP_HUD` _ingamewidget) InteractionName IsHit (`KismetTextLibrary.Conv_TextToString` (`KismetInputLibrary.Key_GetDisplayName` (`|GetArrayItem` _returnvalue))) ModeOfInputUtilisation))))))