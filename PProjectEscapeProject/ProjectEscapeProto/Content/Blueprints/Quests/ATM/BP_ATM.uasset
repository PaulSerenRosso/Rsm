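; Quest ATM that players repair in steps, reusing generator data, widget and sounds.
; On the server, repair delegates drive multicasts that play attached sounds and, after a short delay on each attempt, update the widget's step progress.
; BeginPlay also fires that refresh once and sizes the box from the data's viewing distance.
; Box overlaps toggle widget visibility for prisoner characters.
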(event `self.ReceiveBeginPlay`
  (bind _aswbp_generator_widget (cast `/Game/Blueprints/Widgets/SubWidgets/WBP_GeneratorWidget` (`WidgetComponent.GetWidget` (`self.GeneratorWidget`))))
  (set `self.Widget` _aswbp_generator_widget)
  (`/Engine/EditorBlueprintResources/ActorMacros.Switch Has Authority`
    (:`Authority`
      (add `self.OnRepared` (delegate `Server_Repared`))
      (add `self.OnTryToRepared` (delegate `RefreshWidgetEvent`))
      (`self.RefreshWidgetEvent` null)
      (`self.UpdateBoxCollision`))))

(event `Server_Repared` :!signature `self.OnRepared`
  (params (HitBy :type "Actor Object Reference"))
  (`/Engine/EditorBlueprintResources/ActorMacros.Switch Has Authority`
    (:`Authority`
      (`self.Multicast_Repared`))))

(event `RefreshWidgetEvent` :!signature `self.OnTryToRepared`
  (params (HitBy :type "Actor Object Reference"))
  (`KismetSystemLibrary.Delay` 0.2)
  (`/Engine/EditorBlueprintResources/ActorMacros.Switch Has Authority`
    (:`Authority`
      (`self.Server_TryRepared`))))

(event `Multicast_Repared`
  (`GameplayStatics.SpawnSoundAttached` "/Game/Sounds/SoundCue/A_GeneratorRepared.A_GeneratorRepared" (`self.ItemMesh`) "None" (0.0 0.0 0.0) (struct) "KeepRelativeOffset" false 1.0 1.0 0.0 null null))

(event `Server_TryRepared`
  (`self.Multicast_TryRepared`))

(event `Multicast_TryRepared`
  (`/Game/Blueprints/Widgets/SubWidgets/WBP_GeneratorWidget.UpdateScreen` (`self.Widget`) (`self.currentStep`) (`GeneratorData.MaxStepsToRepare` (`self.GeneratorData`)))
  (`GameplayStatics.SpawnSoundAttached` "/Game/Sounds/SoundCue/A_GeneratorTryRepared.A_GeneratorTryRepared" (`self.ItemMesh`) "None" (0.0 0.0 0.0) (struct) "KeepRelativeOffset" false 1.0 1.0 0.0 null null))

(event `self.Box.OnComponentBeginOverlap`
  (params (OverlappedComponent :type "PrimitiveComponent Object Reference") (OtherActor :type "Actor Object Reference") (OtherComp :type "PrimitiveComponent Object Reference") (OtherBodyIndex :type Integer) (bFromSweep :type Boolean) (SweepResult :type "HitResult Structure (by ref)"))
  (bind _asbp_prisonner_dd (cast `/Game/Blueprints/Characters/BP_PrisonnerDD` OtherActor))
  (`Prisoner.ChangeVisionOfWidget` _asbp_prisonner_dd (`self.GeneratorWidget`) true))

(event `self.Box.OnComponentEndOverlap`
  (params (OverlappedComponent :type "PrimitiveComponent Object Reference") (OtherActor :type "Actor Object Reference") (OtherComp :type "PrimitiveComponent Object Reference") (OtherBodyIndex :type Integer))
  (bind _asbp_prisonner_dd (cast `/Game/Blueprints/Characters/BP_PrisonnerDD` OtherActor))
  (`Prisoner.ChangeVisionOfWidget` _asbp_prisonner_dd (`self.GeneratorWidget`) false))

(fn `UpdateBoxCollision`
  (bind _box (`self.Box`))
  (bind _distancebeforeseewidget (`GeneratorData.DistanceBeforeSeeWidget` (`self.GeneratorData`)))
  (`BoxComponent.SetBoxExtent` _box (`KismetMathLibrary.MakeVector` _distancebeforeseewidget _distancebeforeseewidget (.z (`BoxComponent.BoxExtent` _box))) true))

(fn `UserConstructionScript`)