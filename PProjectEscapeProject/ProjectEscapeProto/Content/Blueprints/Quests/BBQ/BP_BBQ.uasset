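; BP_BBQ is a barbecue quest actor that takes food from prisoners who walk into its sphere and rewards them with points.
; On overlap, the server checks whether the prisoner's first inventory slot holds a BP_Food item, then awards the points.
; It removes and destroys that food and spawns a fire effect above itself.
; The effect spawns in the authority branch, with no multicast in this graph.
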(event `self.Sphere.OnComponentBeginOverlap`
  (params (OverlappedComponent :type "PrimitiveComponent Object Reference") (OtherActor :type "Actor Object Reference") (OtherComp :type "PrimitiveComponent Object Reference") (OtherBodyIndex :type Integer) (bFromSweep :type Boolean) (SweepResult :type "HitResult Structure (by ref)"))
  (bind _returnvalue_location (`KismetMathLibrary.BreakTransform` (`KismetMathLibrary.MakeTransform` (+ (`self.K2_GetActorLocation`) (0.0 0.0 130.0)))))
  (`/Engine/EditorBlueprintResources/ActorMacros.Switch Has Authority`
    (:`Authority`
      (bind _asbp_prisonner_dd (cast `/Game/Blueprints/Characters/BP_PrisonnerDD` OtherActor))
      (bind _inventory (`Prisoner.Inventory` _asbp_prisonner_dd))
      (bind _firstitemslot (`InventorySystem.FirstItemSlot` _inventory))
      (bind _asbp_food (cast `/Game/Blueprints/Quests/BBQ/BP_Food` _firstitemslot))
      (`Prisoner.AddPointToPlayer` _asbp_prisonner_dd 150)
      (`/Engine/EditorBlueprintResources/StandardMacros.IsValid` _asbp_food
        (:`Is Valid`
          (`InventorySystem.TryRemoveItem` _inventory _firstitemslot _asbp_prisonner_dd true 100.0)
          (`self.K2_DestroyActor` _asbp_food)
          (`GameplayStatics.SpawnEmitterAtLocation` "/Game/StarterContent/Particles/P_Fire.P_Fire" _returnvalue_location))))))

(fn `UserConstructionScript`)