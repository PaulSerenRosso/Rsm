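; Balloon-pumping quest task where a prisoner at a task slot presses interact to inflate a balloon against steady pressure decay.
; Holding Progression between min and max runs a validation Timeline that spawns a balloon item into their inventory; that item's finished event completes the task.
; Overpumping multicasts an explosion and makes server noise.
; Progression's RepNotify drives balloon scale and gauge rotation, while the Timeline fills the player's progress bar.
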(event `self.BoxMarker.OnComponentBeginOverlap`
  (params (OverlappedComponent :type "PrimitiveComponent Object Reference") (OtherActor :type "Actor Object Reference") (OtherComp :type "PrimitiveComponent Object Reference") (OtherBodyIndex :type Integer) (bFromSweep :type Boolean) (SweepResult :type "HitResult Structure (by ref)"))
  (bind _returnvalue (`WidgetComponent.GetWidget` (`self.Marker`)))
  ;[0 0 0] MARKER WIDGET FADE
  (if (`self.IsActive`)
    (bind _asbp_prisonner_dd (cast `/Game/Blueprints/Characters/BP_PrisonnerDD` OtherActor))
    (if (`KismetSystemLibrary.IsValid` _asbp_prisonner_dd)
      (bind _aswbp_marker (cast `/Game/Blueprints/Widgets/WBP_Marker` _returnvalue))
      (`UserWidget.PlayAnimation` _returnvalue (`/Game/Blueprints/Widgets/WBP_Marker.Fade` _aswbp_marker) 0.0 1 "Forward" 1.0 false))))

(event `self.BoxMarker.OnComponentEndOverlap`
  (params (OverlappedComponent :type "PrimitiveComponent Object Reference") (OtherActor :type "Actor Object Reference") (OtherComp :type "PrimitiveComponent Object Reference") (OtherBodyIndex :type Integer))
  (bind _returnvalue (`WidgetComponent.GetWidget` (`self.Marker`)))
  ;[0 0 0] MARKER WIDGET FADE
  (if (`self.IsActive`)
    (bind _asbp_prisonner_dd (cast `/Game/Blueprints/Characters/BP_PrisonnerDD` OtherActor))
    (if (`KismetSystemLibrary.IsValid` _asbp_prisonner_dd)
      (bind _aswbp_marker (cast `/Game/Blueprints/Widgets/WBP_Marker` _returnvalue))
      (`UserWidget.PlayAnimation` _returnvalue (`/Game/Blueprints/Widgets/WBP_Marker.Fade` _aswbp_marker) 0.0 1 "Reverse" 1.0 false))))

(event `self.ReceiveBeginPlay`
  (bind (_asbp_task_slot_01 _bsuccess) (cast `/Game/Blueprints/Quests/BP_TaskSlot_01` (`ChildActorComponent.ChildActor` (`self.Slot_01`)) :!pure true))
  ;[0 0 0] MARKER WIDGET
  (bind _aswbp_marker (cast `/Game/Blueprints/Widgets/WBP_Marker` (`WidgetComponent.GetWidget` (`self.Marker`))))
  (set `/Game/Blueprints/Widgets/WBP_Marker.OriginLocation` (`self.K2_GetActorLocation`) _aswbp_marker)
  (bind _returnvalue (message `IInteractable.GetInteractionName` (`ChildActorComponent.ChildActor` (`self.Slot_01`))))
  (set `/Game/Blueprints/Widgets/WBP_Marker.Task` (`self.Pump`) _aswbp_marker)
  (set `self.Progression` 0.0)
  (`SceneComponent.SetRelativeScale3D` (`self.Balloon`) (0.0 0.0 0.0))
  ;[0 0 0] SETUP
  (`TimelineComponent.SetPlayRate` (`self.Timeline`) (/ 1.0 (`self.TimeRateValidation`)))
  (set `self.BalloonPos` (`SceneComponent.K2_GetComponentToWorld` (`self.Balloon`)))
  (if _bsuccess
    (set `self.As BP Task Slot 01` _asbp_task_slot_01)
    ;[0 0 0] BindBlownEvent
    (add `TaskSlot.OnPlayerPressInteractBP` (`self.As BP Task Slot 01`) (delegate `Blown Balloon`))
    ;[0 0 0] OnPlayerEnter
    (add `TaskSlot.OnPlayerEnterSlotBP` (`self.As BP Task Slot 01`) (delegate `OnPlayerEnterSlotBP_Event`))
    ;[0 0 0] OnPlayerExit
    (add `TaskSlot.OnPlayerExitSlotBP` (`self.As BP Task Slot 01`) (delegate `OnPlayerExitSlotBP_Event`))))

(event `OnPlayerEnterSlotBP_Event`
  ;[0 0 0] OnPlayerEnter
  (bind _returnvalue (`|CreateWidget` "/Game/Blueprints/Widgets/WBP_TaskWidget.WBP_TaskWidget_C"))
  (bind _output_get (set `self.TaskWidget` _returnvalue))
  (`UserWidget.AddToViewport` _output_get 0))

(event `Blown Balloon`
  ;[0 0 0] BindBlownEvent
  (`self.Server_BlownBalloon`))

(event `OnPlayerExitSlotBP_Event`
  (bind _taskwidget (`self.TaskWidget`))
  ;[0 0 0] OnPlayerExit
  (`/Engine/EditorBlueprintResources/StandardMacros.IsValid` _taskwidget
    (:`Is Valid`
      (`Widget.RemoveFromParent` _taskwidget)
      (set `self.Progression` 0.0)
      (`self.SetScale` 0.0)
      (`self.SetRotation` 0.0))))

(event `self.ReceiveTick`
  (params (DeltaSeconds :type "Float (single-precision)"))
  (bind (_returnvalue_location _returnvalue_rotation) (`KismetMathLibrary.BreakTransform` (`SceneComponent.K2_GetComponentToWorld` (`self.SpawnerPos`))))
  (bind _returnvalue (- (`self.Progression`) (`self.RatioDecrease`)))
  (bind _asbp_task_slot_01 (cast `/Game/Blueprints/Quests/BP_TaskSlot_01` (`ChildActorComponent.ChildActor` (`self.Slot_01`)) :!pure true))
  (bind _returnvalue_2 (`FunctionsUtilities.Server_GetPlayerWithId` self (`TaskSlot.OccupyingPrisoner` _asbp_task_slot_01)))
  ;[0 0 0] Tick Event
  (`/Engine/EditorBlueprintResources/ActorMacros.Switch Has Authority`
    (:`Authority`
      (`/Engine/EditorBlueprintResources/StandardMacros.IsValid` (`self.As BP Task Slot 01`)
        (:`Is Valid`
          (if (> (`self.Progression`) (- 0.0 (`self.RatioDecrease`)))
            (`|ExecutionSequence`
              (:`then_0`
                (if (and (> (`self.Progression`) (`self.BalloonProgressionMin`)) (< (`self.Progression`) (`self.BalloonProgressionMax`))) :!label _label
                  (bind (_direction _lerp) (`Timeline|Timeline` :!label _label_2)
                    (:`Update`
                      (`self.SetProgressBar` _lerp))
                    (:`Finished`
                      ;[0 0 0] AvoidSpawnWhileExplose
                      (if (> (`self.Progression`) 0.0)
                        ;[0 0 0] Balloon Spawned
                        (set `self.Progression` 0.0)
                        (`self.SetProgressBar` 0.0)
                        (`self.SetScale` 0.0)
                        (`self.SetRotation` 0.0)
                        (`/Engine/EditorBlueprintResources/ActorMacros.Switch Has Authority`
                          (:`Authority`
                            (bind _returnvalue_3 (`|SpawnActorFromClass` "/Game/Blueprints/Objects/Items/BP_Item_Balloon.BP_Item_Balloon_C" (`KismetMathLibrary.MakeTransform` _returnvalue_location _returnvalue_rotation) "Undefined" "MultiplyWithRoot" null null))
                            (`KismetSystemLibrary.Delay` 0.2)
                            (add `Balloon.OnBalloonFinished` _returnvalue_3 (delegate `OnBalloonFinished_Event`))
                            (`InventorySystem.TryAddItem` (`Prisoner.Inventory` _returnvalue_2) _returnvalue_3 _returnvalue_2 true))
                          (:`Remote`
                            _))
                        (`TaskSlot.ServerExitSlot` _asbp_task_slot_01))))
                  (else
                    (goto _label_2 :!via `SetNewTime`))))
              (:`then_1`
                (`KismetSystemLibrary.Delay` 0.1)
                (set `self.Progression` (select `bool` (> _returnvalue 0.0) :`true` _returnvalue :!type "Float (single-precision)"))))))))
    (:`Remote`
      (goto _label))))

(event `OnBalloonFinished_Event`
  (params (WithSuccess :type Boolean))
  ;[0 0 0] Balloon Spawned
  (`self.OnTaskCompleted`))

(event `Server_BlownBalloon`
  ;[0 0 0] EventBlownBalloon
  ;;[1 1 1] AVOID DUPLICATION
  (`KismetSystemLibrary.Delay` (stale `self.ReceiveTick` DeltaSeconds))
  (set `self.Progression` (+ (`self.Progression`) (`self.RatioIncrease`)))
  (if (> (`self.Progression`) (`self.BalloonProgressionMax`))
    (`self.Multicast_ExplodedBalloon`)
    (set `self.Progression` 0.0)
    (`self.SetScale` 0.0)
    (`self.SetRotation` 0.0)
    (`FunctionsUtilities.Server_MakeNoise` self self (`self.K2_GetActorLocation`) 800.0 30000)))

(event `Multicast_ExplodedBalloon`
  ;[0 0 0] EventBlownBalloon
  (`self.SetBalloonExplose`))

(event `self.BP_DeactivateInteraction`
  ;[0 0 0] Hide Widget
  (`SceneComponent.SetVisibility` (`self.Marker`) false false))

(fn `OnRep_Progression`
  (`self.SetScale` (`self.Progression`))
  (`self.SetRotation` (`self.Progression`)))

(fn `SetBalloonExplose`
  (`GameplayStatics.PlaySound2D` "/Game/Sounds/SoundCue/A_BalloonExplosed.A_BalloonExplosed" 1.0 1.0 0.0 null null)
  (bind _returnvalue (`AddComponent|NODE_AddNiagaraComponent-0` :`RelativeTransform` (`SceneComponent.GetRelativeTransform` (`self.Balloon`))))
  (`NiagaraComponent.SetAutoDestroy` _returnvalue false)
  (`SceneComponent.K2_AddLocalOffset` _returnvalue (0.0 0.0 50.0) false false))

(fn `SetProgressBar`
  (params (Progress :type "Float (double-precision)"))
  (bind _taskwidget (`self.TaskWidget`))
  (`/Engine/EditorBlueprintResources/StandardMacros.IsValid` _taskwidget
    (:`Is Valid`
      (`ProgressBar.SetPercent` (`/Game/Blueprints/Widgets/WBP_TaskWidget.YellowProgressBar` _taskwidget) Progress))))

(fn `SetRotation`
  (params (Progression :type "Float (double-precision)"))
  (bind _as_bp_task_slot_01 (`self.As BP Task Slot 01`))
  (bind _gauge (`/Game/Blueprints/Quests/BP_TaskSlot_01.Gauge` _as_bp_task_slot_01))
  (bind (_relativerotation_roll _relativerotation_pitch _relativerotation_yaw) (`KismetMathLibrary.BreakRotator` (`SceneComponent.RelativeRotation` _gauge)))
  (`/Engine/EditorBlueprintResources/StandardMacros.IsValid` _as_bp_task_slot_01
    (:`Is Valid`
      (`SceneComponent.K2_SetRelativeRotation` _gauge (`KismetMathLibrary.MakeRotator` _relativerotation_roll _relativerotation_pitch (`KismetMathLibrary.FInterpTo` _relativerotation_yaw (* Progression 190.0) 0.1 25.0)) false false))))

(fn `SetScale`
  (params (Progression :type "Float (double-precision)"))
  (bind _balloon (`self.Balloon`))
  (bind _relativescale3d_x (`KismetMathLibrary.BreakVector` (`SceneComponent.RelativeScale3D` _balloon)))
  (bind _returnvalue (`KismetMathLibrary.FInterpTo` _relativescale3d_x (`KismetMathLibrary.FClamp` (/ Progression (`self.BalloonProgressionMin`))) (`GameplayStatics.GetWorldDeltaSeconds`) 25.0))
  (`/Engine/EditorBlueprintResources/StandardMacros.IsValid` _balloon
    (:`Is Valid`
      (`SceneComponent.SetRelativeScale3D` _balloon (`KismetMathLibrary.MakeVector` _returnvalue _returnvalue _returnvalue)))))

(fn `UserConstructionScript`)