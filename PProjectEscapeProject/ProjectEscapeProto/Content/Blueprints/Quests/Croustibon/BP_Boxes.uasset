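; Ingredient box for the Croustibon quest that labels itself with the ingredient it represents.
; On BeginPlay, only the authority calls SetLabel, which looks up the DT_Ingredients row named after the IngredientIndex enum value.
; When the row is found, it sets the first material slot of ItemMesh and writes the ingredient's enum value to the TextRender.
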(event `self.ReceiveBeginPlay`
  (`/Engine/EditorBlueprintResources/ActorMacros.Switch Has Authority`
    (:`Authority`
      (`self.SetLabel`))))

(event `SetLabel`
  (`|GetDataTableRow` "/Game/Blueprints/Quests/Croustibon/DT_Ingredients.DT_Ingredients" (`KismetStringLibrary.Conv_StringToName` (`|GetEnumeratorNameAsString` (`self.ingredientIndex`)))
    (:`then`
      (`PrimitiveComponent.SetMaterial` (`self.ItemMesh`) 0 null)
      (`TextRenderComponent.K2_SetText` (`self.TextRender`) (`KismetTextLibrary.Conv_ByteToText` (`self.ingredientIndex`))))))

(fn `UserConstructionScript`)