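; BP_BoxesManager spawns the ingredient boxes at a set of spawn points for the Croustibon quest.
; SpawnAllBoxesInWorld fills one slot per point with the commanded ingredients, pads the rest with random picks from the ingredient reference list, then shuffles them.
; Each entry goes to the SpawnBox event, which spawns a BP_Boxes actor, sets its ingredient index and label, and records it in SpawnedBoxes.
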(event `SpawnBox`
  (params (IndexOfBox :type Integer) (Type :type "/Game/Blueprints/Enums/E_Ingredient Enum" :default "NewEnumerator0"))
  (if (> (`KismetArrayLibrary.Array_Length` (`self.spawnPoints`)) 0)
    (set `self.currentIngredientIndex` Type)
    (bind _returnvalue (`|SpawnActorFromClass` "/Game/Blueprints/Quests/Croustibon/BP_Boxes.BP_Boxes_C" (`KismetMathLibrary.Conv_VectorToTransform` (`self.K2_GetActorLocation` (`|GetArrayItem` (`self.spawnPoints`) IndexOfBox))) "Undefined" "MultiplyWithRoot" null null))
    (set `/Game/Blueprints/Quests/Croustibon/BP_Boxes.ingredientIndex` (`self.currentIngredientIndex`) _returnvalue)
    (`/Game/Blueprints/Quests/Croustibon/BP_Boxes.SetLabel` _returnvalue)
    (`KismetArrayLibrary.Array_Add` (`self.spawnedBoxes`))
    (`KismetSystemLibrary.PrintString` "added box")))

(fn `Spawn All Boxes in World`
  (params (Commands :type "Array of /Game/Blueprints/Enums/E_Ingredient Enum") (IngredientsRef :type "Array of /Game/Blueprints/Enums/E_Ingredient Enum"))
  (locals (CurrentIngredientToSpawn :type "/Game/Blueprints/Enums/E_Ingredient Enum") (CommandToSpawn :type "Array of /Game/Blueprints/Enums/E_Ingredient Enum"))
  (bind _commandtospawn (`local.CommandToSpawn`))
  (for _index (range (`KismetArrayLibrary.Array_Length` (`self.spawnPoints`)))
    (if (< _index (`KismetArrayLibrary.Array_Length` (`local.Commands`)))
      (set `local.CurrentIngredientToSpawn` (`|GetArrayItem` (`local.Commands`) _index))
      (else
        (set `local.CurrentIngredientToSpawn` (`KismetArrayLibrary.Array_Random` (`local.IngredientsRef`)))))
    (`KismetArrayLibrary.Array_Add` (`local.CommandToSpawn`) (`local.CurrentIngredientToSpawn`)))
  (`KismetArrayLibrary.Array_Shuffle` _commandtospawn)
  (for (_array_element _array_index) _commandtospawn
    (`self.SpawnBox` _array_index _array_element)))

(fn `UserConstructionScript`)