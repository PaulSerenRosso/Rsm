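; Dancefloor quest actor that runs a light-and-music show while the task is active, with a marker widget that fades as BP_PrisonnerDD enters or leaves its box.
; The started event turns on the spotlight and music once, then a self-calling delay loop randomizes the light color.
; The finished event ends the loop, shutting off light and music, and multicasts a completion sound.
; Direct interaction is disabled, as CanInteract always returns false.
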(event `self.BoxMarker.OnComponentBeginOverlap`
  (params (OverlappedComponent :type "PrimitiveComponent Object Reference") (OtherActor :type "Actor Object Reference") (OtherComp :type "PrimitiveComponent Object Reference") (OtherBodyIndex :type Integer) (bFromSweep :type Boolean) (SweepResult :type "HitResult Structure (by ref)"))
  (bind _returnvalue (`WidgetComponent.GetWidget` (`self.Marker`)))
  ;[0 0 0] MARKER WIDGET FADE
  (bind _asbp_prisonner_dd (cast `/Game/Blueprints/Characters/BP_PrisonnerDD` OtherActor))
  (if (`KismetSystemLibrary.IsValid` _asbp_prisonner_dd)
    (bind _aswbp_marker (cast `/Game/Blueprints/Widgets/WBP_Marker` _returnvalue))
    (`UserWidget.PlayAnimation` _returnvalue (`/Game/Blueprints/Widgets/WBP_Marker.Fade` _aswbp_marker) 0.0 1 "Forward" 1.0 false)))

(event `self.BoxMarker.OnComponentEndOverlap`
  (params (OverlappedComponent :type "PrimitiveComponent Object Reference") (OtherActor :type "Actor Object Reference") (OtherComp :type "PrimitiveComponent Object Reference") (OtherBodyIndex :type Integer))
  (bind _returnvalue (`WidgetComponent.GetWidget` (`self.Marker`)))
  ;[0 0 0] MARKER WIDGET FADE
  (bind _asbp_prisonner_dd (cast `/Game/Blueprints/Characters/BP_PrisonnerDD` OtherActor))
  (if (`KismetSystemLibrary.IsValid` _asbp_prisonner_dd)
    (bind _aswbp_marker (cast `/Game/Blueprints/Widgets/WBP_Marker` _returnvalue))
    (`UserWidget.PlayAnimation` _returnvalue (`/Game/Blueprints/Widgets/WBP_Marker.Fade` _aswbp_marker) 0.0 1 "Reverse" 1.0 false)))

(event `StartDanceFloor`
  (`/Engine/EditorBlueprintResources/StandardMacros.DoOnce` false
    (:`Completed`
      ;[0 0 0] START FUNCTIONS
      (`self.SetLights` true 500.0)
      (`AudioComponent.SetSound` (`self.MusicSocket`) (`self.Music`))
      (`AudioComponent.Play` (`self.MusicSocket`) 0.0)
      ;[0 0 0] LOOP
      (`self.EventLoop`))))

(event `EventEnd`
  ;[0 0 0] END EVENTS
  (`self.SetLights` false)
  (`AudioComponent.Stop` (`self.MusicSocket`)))

(event `self.ReceiveBeginPlay`
  (`self.SetLights` false)
  ;[0 0 0] MARKER WIDGET
  (bind _aswbp_marker (cast `/Game/Blueprints/Widgets/WBP_Marker` (`WidgetComponent.GetWidget` (`self.Marker`))))
  (set `/Game/Blueprints/Widgets/WBP_Marker.OriginLocation` (`self.K2_GetActorLocation`) _aswbp_marker)
  (bind _returnvalue (message `IInteractable.GetInteractionName` self))
  (set `/Game/Blueprints/Widgets/WBP_Marker.Task` (`self.Name`) _aswbp_marker)
  ;[0 0 0] EVENT FINISHED
  (add `self.OnDancefloorFinished` (delegate `OnDancefloorFinished_EventBP`))
  (add `self.OnDancefloorStarted` (delegate `OnDancefloorStarted_Event`)))

(event `EventLoop`
  ;[0.3021 0 0] EVENT LOOP
  (`KismetSystemLibrary.Delay` 0.2)
  (`LightComponent.SetLightColor` (`self.SpotLight`) (`KismetMathLibrary.Conv_VectorToLinearColor` (`KismetMathLibrary.RandomUnitVector`)) true)
  (if (`self.Loop`)
    (`self.EventLoop`)
    (else
      (`self.EventEnd`))))

(event `OnDancefloorStarted_Event`
  ;[0 0 0] EVENT FINISHED
  (`self.StartDanceFloor`))

(event `OnDancefloorFinished_EventBP`
  ;[0 0 0] EVENT FINISHED
  (set `self.Loop` false)
  (`self.Multicast_OnDancefloorFinished_EventBP`))

(event `Multicast_OnDancefloorFinished_EventBP`
  ;[0 0 0] EVENT FINISHED
  (`GameplayStatics.PlaySoundAtLocation` "/Game/Sounds/SoundCue/A_TaskCompleted.A_TaskCompleted" (`SceneComponent.K2_GetComponentLocation` (`self.Socket_01`)) (struct) 1.0 1.0 0.0 null null null null))

(event `self.BP_DeactivateInteraction`
  ;[0 0 0] Hide Widget
  (`SceneComponent.SetVisibility` (`self.Marker`) false false))

(fn `CanInteract`
  (params (Actor :type "Actor Object Reference"))
  (returns (ReturnValue :type Boolean))
  (return false))

(fn `SetLights`
  (params (bNewVisibility :type Boolean) (NewIntensity :type "Float (single-precision)"))
  (`LightComponent.SetIntensity` (`self.SpotLight`) NewIntensity))

(fn `UserConstructionScript`
  (`SceneComponent.K2_AttachToComponent` (`self.InteractionRoot`) (`self.ItemMesh`) "None" "KeepRelative" "KeepRelative" "KeepRelative" true)
  (`SceneComponent.K2_AttachToComponent` (`self.InteractionSphere`) (`self.InteractionRoot`) "None" "KeepRelative" "KeepRelative" "KeepRelative" true))