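; Numbered table stand (chevalet) for the food tray delivery quest, where prisoners bring trays to the matching table.
; On BeginPlay it sets its material and number text from DT_Chevalet using NumberIndex, and finds the ChevaletManager.
; On server-side box overlap, a prisoner's first-slot tray with a matching table index is removed and destroyed.
; The delivery then awards points and notifies the tray's dispenser and the manager.
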(event `self.ReceiveBeginPlay`
  (`self.SetNumber`)
  (bind _returnvalue (`GameplayStatics.GetActorOfClass` "/Game/Blueprints/Quests/Plateaux/BP_ChevaletManager.BP_ChevaletManager_C"))
  (set `self.ChevaletManager` _returnvalue))

(event `SetNumber`
  ;[1 1 1] INFORMATIONS DES CHEVALETS
  (bind _returnvalue (`|GetDataTableRow` "/Game/Blueprints/Quests/Plateaux/DT_Chevalet.DT_Chevalet" (`KismetStringLibrary.Conv_StringToName` (`KismetStringLibrary.Conv_IntToString` (`self.numberIndex`))))
    (:`then`
      (`PrimitiveComponent.SetMaterial` (`self.Cube`) 0 (`.Texture_11_109EF22945B88F5E8E6973932909833F` (break `/Game/Blueprints/Quests/Plateaux/STRUCT_Chevalet` _returnvalue)))
      (`PrimitiveComponent.SetMaterial` (`self.Cube1`) 0 (`.Texture_11_109EF22945B88F5E8E6973932909833F` (break `/Game/Blueprints/Quests/Plateaux/STRUCT_Chevalet` _returnvalue)))
      (`SceneComponent.K2_SetRelativeLocation` (`self.Cube`) (0.0 0.0 10.0) false false)
      (`SceneComponent.K2_SetRelativeRotation` (`self.Cube`) (struct :`Yaw` 90.0 :`Roll` 65.0) false false)
      (`TextRenderComponent.K2_SetText` (`self.TextRender`) (`KismetTextLibrary.Conv_IntToText` (`.Index_5_961303024589457D4901E0867868719F` (break `/Game/Blueprints/Quests/Plateaux/STRUCT_Chevalet` _returnvalue))))
      (`TextRenderComponent.K2_SetText` (`self.TextRender1`) (`KismetTextLibrary.Conv_IntToText` (`.Index_5_961303024589457D4901E0867868719F` (break `/Game/Blueprints/Quests/Plateaux/STRUCT_Chevalet` _returnvalue)))))))

(event `self.Box.OnComponentBeginOverlap`
  (params (OverlappedComponent :type "PrimitiveComponent Object Reference") (OtherActor :type "Actor Object Reference") (OtherComp :type "PrimitiveComponent Object Reference") (OtherBodyIndex :type Integer) (bFromSweep :type Boolean) (SweepResult :type "HitResult Structure (by ref)"))
  ;[1 1 1] CHECK SI PLATEAU ET CHEVALET CORRESPONDENT > GIVE POINTS
  (`/Engine/EditorBlueprintResources/ActorMacros.Switch Has Authority`
    (:`Authority`
      (bind _asbp_prisonner_dd (cast `/Game/Blueprints/Characters/BP_PrisonnerDD` OtherActor))
      (bind _inventory (`Prisoner.Inventory` _asbp_prisonner_dd))
      (bind _firstitemslot (`InventorySystem.FirstItemSlot` _inventory))
      (bind _asbp_plateau (cast `/Game/Blueprints/Quests/Plateaux/BP_FoodTray` _firstitemslot))
      (bind _iscorrecttablenumber_ (`self.Check Table` (`/Game/Blueprints/Quests/Plateaux/BP_FoodTray.tableIndex` _asbp_plateau)))
      (if _iscorrecttablenumber_
        (`KismetSystemLibrary.PrintString` "Good table" true true (struct :`R` 0.011239 :`G` 1.0 :`B` 0.202127 :`A` 1.0))
        (`/Engine/EditorBlueprintResources/StandardMacros.IsValid` _asbp_plateau
          (:`Is Valid`
            (`InventorySystem.TryRemoveItem` _inventory _firstitemslot _asbp_prisonner_dd true 100.0)
            (`/Game/Blueprints/Quests/Plateaux/BP_TrayDispenser.TrayDelivered` (`/Game/Blueprints/Quests/Plateaux/BP_FoodTray.OwningDispenser` _asbp_plateau))
            (`self.K2_DestroyActor` _asbp_plateau))
          (:`Is Not Valid`
            _))
        (`Prisoner.AddPointToPlayer` _asbp_prisonner_dd 250)
        (`/Game/Blueprints/Quests/Plateaux/BP_ChevaletManager.PlateauDelivered` (`self.ChevaletManager`))
        (else
          (`KismetSystemLibrary.PrintString` "Wrong table" true true (struct :`R` 1.0 :`B` 0.084041 :`A` 1.0)))))))

(fn `CanInteract`
  (params (Actor :type "Actor Object Reference"))
  (returns (ReturnValue :type Boolean))
  (return false))

(fn `Check Table`
  (params (PlateauIndex :type Integer))
  (returns (`isCorrectTableNumber?` :type Boolean))
  (return (== PlateauIndex (`self.numberIndex`))))

(fn `GetInteractionHoldTime`
  (returns (ReturnValue :type "Float (single-precision)"))
  (return 0.0))

(fn `GetInteractionName`
  (returns (ReturnValue :type String))
  (return ""))

(fn `GetTypeInteractionName`
  (returns (ReturnValue :type String))
  (return ""))

(fn `IsInteractionValid`
  (params (Actor :type "Actor Object Reference"))
  (returns (ReturnValue :type Boolean))
  (return false))

(fn `OnRep_numberIndex`)

(fn `TryInteract`
  (params (Actor :type "Actor Object Reference"))
  (returns (ReturnValue :type Boolean))
  (return false))

(fn `TryStopInteract`
  (params (Actor :type "Actor Object Reference"))
  (returns (ReturnValue :type Boolean))
  (return false))

(fn `UserConstructionScript`)