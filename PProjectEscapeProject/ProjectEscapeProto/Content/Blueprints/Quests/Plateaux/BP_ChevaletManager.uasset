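; Quest manager for the tray (plateau) delivery task, spawning numbered chevalets and tracking deliveries on the server.
; Shortly after BeginPlay, it shuffles its spawn points, clears existing chevalets and spawns one numbered chevalet per point, within a maximum count.
; PlateauDelivered counts deliveries and, at the target, calls EndOfQuests on BP_QuestManager if the success flag is set.
; It does not respawn chevalets, as that dispenser-linked wiring never runs.
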(event `self.ReceiveBeginPlay`
  ;[1 1 1] INSTANTIATION DES CHEVALETS
  (`/Engine/EditorBlueprintResources/ActorMacros.Switch Has Authority`
    (:`Authority`
      (bind _returnvalue (`GameplayStatics.GetActorOfClass` "/Game/Blueprints/Quests/BP_QuestManager.BP_QuestManager_C"))
      (set `self.QuestManager` _returnvalue)
      (`KismetSystemLibrary.Delay` 1.0)
      (`self.PlateauTask` 5.0))))

(event `PlateauTask`
  (params (NumberOfLoop :type "Float (double-precision)" :default 5.0))
  ;[1 1 1] NOMBRE DE FOIS QU'ON PLAY L'EVENT
  (if (!= NumberOfLoop 0.0)
    (`KismetArrayLibrary.Array_Shuffle` (`self.spawnPoints`))
    (`self.RespawnChevalets`)))

(event `RespawnChevalets`
  (bind _spawnedchevalets (`self.spawnedChevalets`))
  ;[1 1 1] DESTRUCTION ET RESPAWN DES CHEVALETS QUAND LIVRAISON
  (for _array_element _spawnedchevalets
    (`/Engine/EditorBlueprintResources/StandardMacros.IsValid` _array_element
      (:`Is Valid`
        (`self.K2_DestroyActor` _array_element))))
  (`KismetArrayLibrary.Array_Clear` _spawnedchevalets)
  (for _index (range (`KismetArrayLibrary.Array_Length` (`self.spawnPoints`)))
    (`self.SpawnChevalet` _index)))

(event `SpawnChevalet`
  (params (IndexOfChevalet :type Integer))
  (bind _returnvalue (`KismetArrayLibrary.Array_Length` (`self.spawnPoints`)))
  ;[1 1 1] APPARITION ET STOCKAGE DES CHEVALETS
  (if (and (<= _returnvalue (`self.maxChevaletCount`)) (> _returnvalue 0))
    (set `self.currentChevaletIndex` (+ IndexOfChevalet 1))
    (bind _returnvalue_2 (`|SpawnActorFromClass` "/Game/Blueprints/Quests/Plateaux/BP_Chevalet.BP_Chevalet_C" (`self.GetTransform` (`|GetArrayItem` (`self.spawnPoints`) IndexOfChevalet)) "Undefined" "MultiplyWithRoot" null null))
    (set `/Game/Blueprints/Quests/Plateaux/BP_Chevalet.numberIndex` (`self.currentChevaletIndex`) _returnvalue_2)
    (`/Game/Blueprints/Quests/Plateaux/BP_Chevalet.SetNumber` _returnvalue_2)
    (`KismetArrayLibrary.Array_Add` (`self.spawnedChevalets`) _returnvalue_2)))

(event `PlateauDelivered`
  (`/Engine/EditorBlueprintResources/ActorMacros.Switch Has Authority`
    (:`Authority`
      (bind _result (`/Engine/EditorBlueprintResources/StandardMacros.IncrementInt` (`self.NumberPlateauDelivered`))
        (:`  `
          (`KismetSystemLibrary.PrintString` (`KismetStringLibrary.Conv_IntToString` _result))
          (if (>= (`self.NumberPlateauDelivered`) (`self.MaxDelivery`))
            (`KismetSystemLibrary.PrintString` "Tache réussie")
            (if (`self.IsSuccessfull`)
              (`QuestManager.EndOfQuests` (`self.QuestManager`) false))))))))

(fn `UserConstructionScript`)