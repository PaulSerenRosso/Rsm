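; Food tray Blueprint for the Plateaux quest that carries a randomly assigned table number shown on its text render.
; On BeginPlay, only the authority rolls an index from 1 to 9 and passes it to the ReplicateGoodIndex event.
; That event stores it as TableIndex, writes it to the text render and prints it to screen.
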(event `self.ReceiveBeginPlay`
  (`/Engine/EditorBlueprintResources/ActorMacros.Switch Has Authority`
    (:`Authority`
      (`self.ReplicateGoodIndex` (+ (`KismetMathLibrary.RandomInteger` 9) 1)))))

(event `ReplicateGoodIndex`
  (params (GoodIndex :type Integer))
  (bind _output_get (set `self.tableIndex` GoodIndex))
  (bind _returnvalue (`KismetTextLibrary.Conv_IntToText` _output_get))
  (`TextRenderComponent.K2_SetText` (`self.TextRender1`) _returnvalue)
  (`KismetSystemLibrary.PrintString` (`KismetTextLibrary.Conv_TextToString` _returnvalue)))

(fn `UserConstructionScript`)