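; Food tray dispenser for a prisoner quest that hands out one tray at a time and completes a task on delivery.
; On the server, a box overlap spawns a BP_FoodTray linked to this dispenser and adds it to the inventory of a prisoner not already holding one.
; A successful pickup turns the dynamic emissive light red, plays a sound and locks the dispenser until TrayDelivered restores green.
; Interaction functions are stubs, so pickup is overlap-only.
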(event `self.ReceiveBeginPlay`
  (bind _returnvalue (`KismetMaterialLibrary.CreateDynamicMaterialInstance` "/Game/Art/Environments/Materials/MaterialInstances/Props/MI_Light_Set_02.MI_Light_Set_02"))
  (bind _output_get (set `self.MID` _returnvalue))
  (`PrimitiveComponent.SetMaterial` (`self.Dispenser`) 0 _output_get)
  (`MaterialInstanceDynamic.SetVectorParameterValue` _output_get "EmissiveColor" (struct :`R` 0.318091 :`G` 0.942708 :`B` 0.19099 :`A` 1.0))
  (`/Engine/EditorBlueprintResources/ActorMacros.Switch Has Authority`
    (:`Authority`
      (`KismetSystemLibrary.PrintString` "Plateau disponible")
      (add `PrimitiveComponent.OnComponentBeginOverlap` (`self.Box`) (delegate `OnComponentBeginOverlap_Event`)))))

(event `OnComponentBeginOverlap_Event`
  (params (OverlappedComponent :type "PrimitiveComponent Object Reference") (OtherActor :type "Actor Object Reference") (OtherComp :type "PrimitiveComponent Object Reference") (OtherBodyIndex :type Integer) (bFromSweep :type Boolean) (SweepResult :type "HitResult Structure (by ref)"))
  (bind _asbp_prisonner_dd (cast `/Game/Blueprints/Characters/BP_PrisonnerDD` OtherActor))
  (`self.SpawnAssignPlateau` _asbp_prisonner_dd))

(event `SpawnAssignPlateau`
  (params (OtherActor :type "/Game/Blueprints/Characters/BP_PrisonnerDD Object Reference"))
  (bind _inventory (`Prisoner.Inventory` OtherActor))
  ;[1 1 1] LIVRAISON DU PLATEAU
  (if (and (`self.AvailablePlateau?`) (not (or (`.bSuccess` (cast `/Game/Blueprints/Quests/Plateaux/BP_FoodTray` (`InventorySystem.FirstItemSlot` _inventory) :!pure true)) (`.bSuccess` (cast `/Game/Blueprints/Quests/Plateaux/BP_FoodTray` (`InventorySystem.SecondItemSlot` _inventory) :!pure true)))))
    (bind _returnvalue (`|SpawnActorFromClass` "/Game/Blueprints/Quests/Plateaux/BP_FoodTray.BP_FoodTray_C" (`SceneComponent.K2_GetComponentToWorld` (`self.SpawnPoint`)) "Undefined" "OverrideRootScale" null null))
    (set `/Game/Blueprints/Quests/Plateaux/BP_FoodTray.OwningDispenser` self _returnvalue)
    (`KismetSystemLibrary.Delay` 0.2)
    (bind _returnvalue_2 (`InventorySystem.TryAddItem` (`Prisoner.Inventory` OtherActor) _returnvalue OtherActor true))
    (if _returnvalue_2
      (`KismetSystemLibrary.PrintString` "Plateau récupéré")
      (`self.UpdateDispenserData_MULTICAST`))
    (else
      (`KismetSystemLibrary.PrintString` "Livrez le plateau en cours"))))

(event `TrayDelivered`
  (set `self.AvailablePlateau?` true)
  (`MaterialInstanceDynamic.SetVectorParameterValue` (`self.MID`) "EmissiveColor" (struct :`R` 0.317647 :`G` 0.941177 :`B` 0.192157 :`A` 1.0))
  (`self.ReplicatedTrayDelivered`)
  (`self.OnTaskCompleted`))

(event `ReplicatedTrayDelivered`
  (set `self.AvailablePlateau?` true)
  (`MaterialInstanceDynamic.SetVectorParameterValue` (`self.MID`) "EmissiveColor" (struct :`R` 0.317647 :`G` 0.941177 :`B` 0.192157 :`A` 1.0)))

(event `UpdateDispenserData_MULTICAST`
  (`MaterialInstanceDynamic.SetVectorParameterValue` (`self.MID`) "EmissiveColor" (struct :`R` 0.942708 :`G` 0.103109 :`B` 0.103109 :`A` 1.0))
  (`GameplayStatics.PlaySoundAtLocation` "/Game/Sounds/SoundWave/A_Borgir.A_Borgir" (`self.SoundLocation`) (struct) 1.0 1.0 0.0 null null null null)
  (set `self.AvailablePlateau?` false))

(fn `CanInteract`
  (params (Actor :type "Actor Object Reference"))
  (returns (ReturnValue :type Boolean))
  (return false))

(fn `GetInteractionHoldTime`
  (returns (ReturnValue :type "Float (single-precision)"))
  (return 0.0))

(fn `GetInteractionName`
  (returns (ReturnValue :type String))
  (return ""))

(fn `GetTypeInteractionName`
  (returns (ReturnValue :type String))
  (return ""))

(fn `IsInteractionValid`
  (params (Actor :type "Actor Object Reference"))
  (returns (ReturnValue :type Boolean))
  (return false))

(fn `OnRep_AvailablePlateau?`)

(fn `TryInteract`
  (params (Actor :type "Actor Object Reference"))
  (returns (ReturnValue :type Boolean))
  (return false))

(fn `TryStopInteract`
  (params (Actor :type "Actor Object Reference"))
  (returns (ReturnValue :type Boolean))
  (return false))

(fn `UserConstructionScript`)